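; Tutorial encyclopedia actor, an interactable clipboard that leads into the open-menu tutorial prompt.
; On BeginPlay it loads the save game and destroys itself if the beginning tutorial checkpoint is already done.
; Interacting plays a timeline that drives the clipboard material's dissolve parameter, then adds the Tutorial_OpenMenu widget to the viewport and destroys the actor.
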(event `self.ReceiveBeginPlay`
  (bind _returnvalue (`GameplayStatics.LoadGameFromSlot` "mySlot"))
  (bind _asmy_save_game (cast `/Game/Blueprints/Important/mySaveGame` _returnvalue))
  (bind _tutorialcheckpoints_beginningtutorialdone_ (break `/Game/Blueprints/Structs/TutorialCheckpointsStruct` (`/Game/Blueprints/Important/mySaveGame.TutorialCheckpoints` _asmy_save_game)))
  (if _tutorialcheckpoints_beginningtutorialdone_
    (`self.K2_DestroyActor`)))

(event `Dissolve`
  (bind (_direction _thing) (`Timeline|d_solve`)
    (:`Update`
      (`MeshComponent.SetScalarParameterValueOnMaterials` (`self.Clipboard`) "DissolveFactor" _thing))
    (:`Finished`
      (bind _returnvalue (`|CreateWidget` "/Game/Blueprints/Widgets/Tutorial_OpenMenu.Tutorial_OpenMenu_C"))
      (`UserWidget.AddToViewport` _returnvalue 0)
      (`self.K2_DestroyActor`))))

(event `/Game/Blueprints/Interact.Interact`
  (`self.Dissolve`))

(fn `UserConstructionScript`)