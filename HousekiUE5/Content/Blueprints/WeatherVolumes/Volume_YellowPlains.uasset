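; Weather volume for the Yellow Plains that shifts the directional sunlight to a yellow look while an actor overlaps it.
; BeginPlay finds directional lights and caches color, intensity and reference from the last one iterated.
; The EnterArea timeline blends that light toward the yellow sun values on overlap begin and reverses on end for a gradual transition.
; Overlaps are not filtered by actor type.
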(event `self.ReceiveBeginPlay`
  (bind _outactors (`GameplayStatics.GetAllActorsOfClass` "/Script/Engine.DirectionalLight"))
  (for _array_element _outactors
    (bind _lightcomponent (`Light.LightComponent` _array_element))
    (set `self.Day Sun Color` (`LightComponentBase.GetLightColor` _lightcomponent))
    (set `self.Day Sun Intensity` (`LightComponentBase.Intensity` _lightcomponent))
    (set `self.Day Sun` _array_element)))

(event `self.ReceiveActorBeginOverlap`
  (params (OtherActor :type "Actor Object Reference"))
  (bind _lightcomponent (`Light.LightComponent` (`self.Day Sun`)))
  ;[1 1 1] Entering/Leaving plays a transition, not instant.
  (bind (_direction _newtrack_0) (`Timeline|EnterArea` :!label _label)
    (:`Update`
      (`LightComponent.SetIntensity` _lightcomponent (`KismetMathLibrary.Lerp` (`self.Day Sun Intensity`) (`self.Yellow Sun Intensity`) _newtrack_0))
      (`LightComponent.SetLightColor` _lightcomponent (`KismetMathLibrary.LinearColorLerp` (`self.Day Sun Color`) (`self.Yellow Sun Color`) _newtrack_0) true))))

(event `self.ReceiveActorEndOverlap`
  (params (OtherActor :type "Actor Object Reference"))
  (goto _label :!via `Reverse`))

(fn `UserConstructionScript`)