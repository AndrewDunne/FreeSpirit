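; Blueprint function library of date-time math helpers, plus shortcuts that return myGameState and the first player's mychara.
; Add and subtract convert DateTimes to total hours through month-length tables, using fixed 8760-hour years and a simple divisible-by-four leap rule.
; HoursToDate rebuilds dates from those hours, and a print helper displays them with month names.
; Some leap-year branches compare against zero or read the non-leap table, unlike their normal-year counterparts.
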(fn `AddDateTime`
  (params (`Date 1` :type "DateTime Structure") (Hours :type "Float (double-precision)"))
  (returns (`Sum (Date)` :type "DateTime Structure"))
  (bind _hours (`self.DateToHours` `Date 1`))
  (bind _date (`self.HoursToDate` (+ _hours Hours)))
  (return _date))

(fn `DateToHours`
  (params (Date :type "DateTime Structure"))
  (returns (Hours :type "Float (double-precision)"))
  (bind (_year _month _day _hour _minute _second) (`KismetMathLibrary.BreakDateTime` Date))
  (bind _number_of_days (`self.Number Of Days So Far in the Year` Date))
  (return (+ (* _year 8760) (* _number_of_days 24) (`KismetMathLibrary.Conv_IntToDouble` _hour) (/ (`KismetMathLibrary.Conv_IntToDouble` _minute) 60.0) (/ (`KismetMathLibrary.Conv_IntToDouble` _second) 3600.0))))

(fn `DaysInCurrentMonth`
  (params (Date :type "DateTime Structure"))
  (returns (NumDays :type Integer))
  (locals (`Days per month` :type "Array of Integer") (`Days per month (leap year)` :type "Array of Integer") (Days :type Integer))
  (bind (_year _month) (`KismetMathLibrary.BreakDateTime` Date))
  (bind _returnvalue (- _month 1))
  (if (== (mod _year 4) 0)
    (set `local.Days` (`|GetArrayItem` (`local.Days per month (leap year)`) _returnvalue))
    (else
      (set `local.Days` (`|GetArrayItem` (`local.Days per month`) _returnvalue))))
  (return (`local.Days`)))

(fn `GMC`
  (returns (myChara :type "/Game/Blueprints/Important/mychara Object Reference"))
  (bind _asmychara (cast `/Game/Blueprints/Important/mychara` (`GameplayStatics.GetPlayerCharacter` null)))
  (return _asmychara))

(fn `GMGS`
  (returns (myGameState :type "/Game/Blueprints/Important/myGameState Object Reference"))
  (bind _asmy_game_state (cast `/Game/Blueprints/Important/myGameState` (`GameplayStatics.GetGameState` null)))
  (return _asmy_game_state))

(fn `HoursToDate`
  (params (Hours :type "Float (double-precision)"))
  (returns (Date :type "DateTime Structure"))
  (bind _returnvalue (* Hours 60.0))
  (bind _returnvalue_2 (`KismetMathLibrary.FTrunc` (/ Hours 8760.0)))
  (bind _returnvalue_3 (/ (mod Hours 8760.0) 24.0))
  (bind _returnvalue_4 (== (mod _returnvalue_2 4) 0))
  (bind _month (`self.Month From Days in Year` (`KismetMathLibrary.FTrunc` _returnvalue_3) _returnvalue_4))
  (bind _days (`self.Num days before start of month` _month _returnvalue_4))
  (return (`KismetMathLibrary.MakeDateTime` _returnvalue_2 _month (`KismetMathLibrary.FTrunc` (- _returnvalue_3 _days)) (`KismetMathLibrary.FTrunc` (mod Hours 24.0)) (`KismetMathLibrary.FTrunc` (mod _returnvalue 60.0)) (`KismetMathLibrary.FTrunc` (mod (* _returnvalue 60.0) 60.0)))))

(fn `Month From Days in Year`
  (params (Days :type Integer) (`LeapYear?` :type Boolean))
  (returns (Month :type Integer))
  (locals (`Days per month` :type "Array of Integer") (`Days per month (leap year)` :type "Array of Integer") (DaysElapsedSoFar :type Integer) (myMonth :type Integer) (`MonthSet?` :type Boolean))
  (if `LeapYear?`
    (for (_array_element _array_index) (`local.Days per month (leap year)`)
      (if (not (`local.MonthSet?`))
        (bind _returnvalue (+ (`local.DaysElapsedSoFar`) _array_element))
        (if (< _returnvalue 0)
          (set `local.DaysElapsedSoFar` _returnvalue)
          (else
            (set `local.myMonth` (+ _array_index 1))
            (set `local.MonthSet?` true)))))
    (else
      (for (_array_element_2 _array_index_2) (`local.Days per month`)
        (if (not (`local.MonthSet?`))
          (bind _returnvalue_2 (+ (`local.DaysElapsedSoFar`) _array_element_2))
          (if (< _returnvalue_2 Days)
            (set `local.DaysElapsedSoFar` _returnvalue_2)
            (else
              (set `local.myMonth` (+ _array_index_2 1))
              (set `local.MonthSet?` true)))))))
  (return (`local.myMonth`)))

(fn `Num days before start of month`
  (params (Month :type Integer) (`LeapYear?` :type Boolean))
  (returns (Days :type Integer))
  (locals (`Days per month` :type "Array of Integer") (`Days per month (leap year)` :type "Array of Integer") (myDays :type Integer))
  (if `LeapYear?`
    (for (_array_element _array_index) (`local.Days per month`)
      (if (< _array_index (- Month 1))
        (set `local.myDays` (+ (`local.myDays`) _array_element))
        (return (`local.myDays`))))
    (else
      (for (_array_element_2 _array_index_2) (`local.Days per month`)
        (if (< _array_index_2 (- Month 1))
          (set `local.myDays` (+ (`local.myDays`) _array_element_2))))))
  (return (`local.myDays`)))

(fn `Number Of Days So Far in the Year`
  (params (Date :type "DateTime Structure"))
  (returns (`Number of days` :type Integer))
  (locals (`Days per month` :type "Array of Integer") (`Days per month (leap year)` :type "Array of Integer") (numDays :type Integer))
  (bind (_year _month _day) (`KismetMathLibrary.BreakDateTime` Date))
  (if (== (mod _year 4) 0)
    (for (_array_element _array_index) (`local.Days per month (leap year)`)
      (if (> 0 (+ _array_index 1))
        (set `local.numDays` (+ _array_element (`local.numDays`)))))
    (else
      (for (_array_element_2 _array_index_2) (`local.Days per month`)
        (if (> _month (+ _array_index_2 1))
          (set `local.numDays` (+ _array_element_2 (`local.numDays`)))))))
  (bind _output_get (set `local.numDays` (+ _day (`local.numDays`))))
  (return _output_get))

(fn `Print Date Time`
  (params (Date :type "DateTime Structure") (Duration :type "Float (double-precision)" :default 10.0))
  (locals (Months :type "Array of String"))
  (bind (_year _month _day _hour _minute _second) (`KismetMathLibrary.BreakDateTime` Date))
  (`KismetSystemLibrary.PrintString` null (`KismetStringLibrary.Concat_StrStr` (`|GetArrayItem` (`local.Months`) (- _month 1)) " " (`KismetStringLibrary.Conv_IntToString` _day) ", " (`KismetStringLibrary.Conv_IntToString` _year) ". " (`KismetStringLibrary.Conv_IntToString` _hour) ":" (`KismetStringLibrary.Conv_IntToString` _minute) ":" (`KismetStringLibrary.Conv_IntToString` _second)) true true (struct :`G` 0.66 :`B` 1.0 :`A` 1.0) Duration))

(fn `SubtractDateTime`
  (params (`Date 1` :type "DateTime Structure") (`Date 2` :type "DateTime Structure"))
  (returns (`Difference (Hours)` :type "Float (double-precision)"))
  (bind _hours (`self.DateToHours` `Date 1`))
  (bind _hours_2 (`self.DateToHours` `Date 2`))
  (return (- _hours _hours_2)))