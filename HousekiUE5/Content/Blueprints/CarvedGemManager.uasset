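; CarvedGemManager keeps the collection of carved geodes, along with a set of decoration geodes restored from the save game.
; On BeginPlay it loads both lists from the "mySlot" save and prints each carved geode's mineral name to screen.
; NewCarvedGem appends a geode and drops the oldest once CarvedGemCapacity is exceeded, without writing back to the save.
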(event `self.ReceiveBeginPlay`
  ;[1 1 1] Loading from SaveGame
  (bind _returnvalue (`GameplayStatics.LoadGameFromSlot` "mySlot"))
  (bind _asmy_save_game (cast `/Game/Blueprints/Important/mySaveGame` _returnvalue))
  (bind _carvedgeodes (`/Game/Blueprints/Important/mySaveGame.CarvedGeodes` _asmy_save_game))
  (set `self.CarvedGeodes` _carvedgeodes)
  (set `self.DecorationGeodes` (`/Game/Blueprints/Important/mySaveGame.DecorationGeodes` _asmy_save_game))
  (for _array_element _carvedgeodes
    (`KismetSystemLibrary.PrintString` (`KismetStringLibrary.Conv_NameToString` (`.MineralName_31_8AFEAFE54500487AED9CE78F34B44BE9` (break `/Game/Blueprints/Structs/GeodeStruct` _array_element))) true true (struct :`G` 0.66 :`B` 1.0 :`A` 1.0) 33.0)))

(fn `NewCarvedGem`
  (params (`New Geode` :type "/Game/Blueprints/Structs/GeodeStruct Structure"))
  (`KismetArrayLibrary.Array_Add` (`self.CarvedGeodes`) `New Geode`)
  (if (> (`KismetArrayLibrary.Array_Length` (`self.CarvedGeodes`)) (`self.CarvedGemCapacity`))
    (`KismetArrayLibrary.Array_Remove` (`self.CarvedGeodes`))))

(fn `UserConstructionScript`)