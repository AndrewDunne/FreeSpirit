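; Tutorial manager that triggers the game's one-time beginning and memory tutorials.
; On BeginPlay it binds to GameState and player character events, then plays the startup cutscene if the loaded save lacks the beginning-tutorial flag.
; The first memory found toggles the player's menu.
; Completion flags are set in GameState's TutorialCheckpoints struct, including when the encyclopedia popup closes; this Blueprint does not save them.
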(event `self.ReceiveBeginPlay`
  (bind _mygamestate (`/Game/Blueprints/MyFunctionLibrary.GMGS`))
  (set `self.GameState` _mygamestate)
  (bind _mychara (`/Game/Blueprints/MyFunctionLibrary.GMC`))
  (set `self.myChara` _mychara)
  (add `/Game/Blueprints/Important/myGameState.memoryFound` (`self.GameState`) (delegate `Memory Found`))
  (add `/Game/Blueprints/Important/mychara.EncyclopediaTutorialPopupClosed` (`self.myChara`) (delegate `Beginning tutorial complete`))
  (bind _returnvalue (`GameplayStatics.LoadGameFromSlot` "mySlot"))
  (bind _asmy_save_game (cast `/Game/Blueprints/Important/mySaveGame` _returnvalue))
  (bind _tutorialcheckpoints_beginningtutorialdone_ (break `/Game/Blueprints/Structs/TutorialCheckpointsStruct` (`/Game/Blueprints/Important/mySaveGame.TutorialCheckpoints` _asmy_save_game)))
  (if (not _tutorialcheckpoints_beginningtutorialdone_)
    (bind _asmychara (cast `/Game/Blueprints/Important/mychara` (`GameplayStatics.GetPlayerCharacter` 0)))
    (`/Game/Blueprints/Important/mychara.StartupCutscene` _asmychara)))

(event `Memory Found`
  (bind (_tutorialcheckpoints_beginningtutorialdone_ _tutorialcheckpoints_memorytutorialdone_) (break `/Game/Blueprints/Structs/TutorialCheckpointsStruct` (`/Game/Blueprints/Important/myGameState.TutorialCheckpoints` (`self.GameState`))))
  (`KismetSystemLibrary.PrintString` "Mem found!")
  (if (not _tutorialcheckpoints_memorytutorialdone_)
    (`/Game/Blueprints/Important/mychara.ToggleMenu` (`self.myChara`) 1)
    (setmembers `/Game/Blueprints/Structs/TutorialCheckpointsStruct` :`StructRef` (`/Game/Blueprints/Important/myGameState.TutorialCheckpoints` (`self.GameState`)) :`MemoryTutorialDone?` true)))

(event `Beginning tutorial complete`
  (setmembers `/Game/Blueprints/Structs/TutorialCheckpointsStruct` :`StructRef` (`/Game/Blueprints/Important/myGameState.TutorialCheckpoints` (`self.GameState`)) :`BeginningTutorialDone?` true))

(fn `UserConstructionScript`)