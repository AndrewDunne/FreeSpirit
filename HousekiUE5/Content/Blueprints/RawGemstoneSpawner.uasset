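; Actor that spawns a RawGemstone into a free RawGemstoneSocket after a timed interval, with its mesh acting as a growth indicator.
; BeginPlay sets the next spawn time and starts a one-second looping timer that scales the mesh by elapsed time.
; When time is up, it attaches a gem to the first empty socket, marks it occupied and reschedules.
; GemSpawned is never reset here, limiting spawning to one gem.
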(event `self.ReceiveBeginPlay`
  (`self.Set Next Spawn Time`)
  (`KismetSystemLibrary.K2_SetTimer` null "AdjustRawGemSize" 1.0 true)
  (bind _difference__hours_ (`/Game/Blueprints/MyFunctionLibrary.SubtractDateTime` (`KismetMathLibrary.Now`) (`self.Next Spawn Time`)))
  (if (> _difference__hours_ 0.0)
    (`self.Spawn Gemstone`)))

(fn `AdjustRawGemSize`
  (bind _difference__hours_ (`/Game/Blueprints/MyFunctionLibrary.SubtractDateTime` (`KismetMathLibrary.Now`) (`self.Next Spawn Time`)))
  (`SceneComponent.SetRelativeScale3D` (`self.StaticMesh`) (`KismetMathLibrary.Conv_DoubleToVector` (+ (/ _difference__hours_ (`self.TimeInterval`)) 1.0)))
  (bind _difference__hours__2 (`/Game/Blueprints/MyFunctionLibrary.SubtractDateTime` (`KismetMathLibrary.Now`) (`self.Next Spawn Time`)))
  (if (> _difference__hours__2 0.0)
    (`self.Spawn Gemstone`)
    (`self.Set Next Spawn Time`)))

(fn `Set Next Spawn Time`
  (bind _sum__date_ (`/Game/Blueprints/MyFunctionLibrary.AddDateTime` (`KismetMathLibrary.Now`) (`self.TimeInterval`)))
  (set `self.Next Spawn Time` _sum__date_))

(fn `Spawn Gemstone`
  (locals (GemSpawned :type Boolean))
  (bind _outactors (`GameplayStatics.GetAllActorsOfClass` "/Game/Blueprints/RawGemstoneSocket.RawGemstoneSocket_C"))
  (for _array_element _outactors
    (if (`local.GemSpawned`)
      _
      (elif (not (`/Game/Blueprints/RawGemstoneSocket.HasGem?` _array_element))
        (set `local.GemSpawned` true)
        (bind _returnvalue (`|SpawnActorFromClass` "/Game/Blueprints/RawGemstone.RawGemstone_C" (`self.GetTransform`) "Undefined" "OverrideRootScale" null null))
        (`self.K2_AttachToActor` _returnvalue _array_element "None" "SnapToTarget" "KeepRelative" "KeepRelative" true)
        (set `/Game/Blueprints/RawGemstoneSocket.HasGem?` true _array_element)
        (`/Game/Blueprints/MyFunctionLibrary.Print Date Time` (`self.Next Spawn Time`) 5.0)
        (`KismetSystemLibrary.PrintString` "Next gem spawning at:" true true (struct :`G` 0.66 :`B` 1.0 :`A` 1.0) 5.0)))))

(fn `UserConstructionScript`)