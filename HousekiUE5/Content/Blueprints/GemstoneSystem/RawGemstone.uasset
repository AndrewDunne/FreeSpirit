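; RawGemstone is a Blueprint in the gemstone system that displays a raw gemstone using a configurable mesh and material.
; The Construction Script applies the Mesh and Material variables to RawGemstoneMesh, setting the material on the first slot.
; BeginPlay repeats the same assignment when play starts.
; The graphs contain no other gameplay logic.
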(event `self.ReceiveBeginPlay`
  (bind _rawgemstonemesh (`self.RawGemstoneMesh`))
  (`StaticMeshComponent.SetStaticMesh` _rawgemstonemesh (`self.Mesh`))
  (`PrimitiveComponent.SetMaterial` _rawgemstonemesh 0 (`self.Material`)))

(fn `UserConstructionScript`
  (bind _rawgemstonemesh (`self.RawGemstoneMesh`))
  (`StaticMeshComponent.SetStaticMesh` _rawgemstonemesh (`self.Mesh`))
  (`PrimitiveComponent.SetMaterial` _rawgemstonemesh 0 (`self.Material`)))