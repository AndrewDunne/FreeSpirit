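; Geode actor for a gem-cutting minigame that copies a static mesh into a procedural mesh the player carves with plane slices.
; Clicks trace from cursor or view center for spherical or vertical facet cuts, while knife-project mode cuts along a dragged line drawn in a SculptUI widget.
; Non-world geodes rotate with right-drag.
; After non-faceting click cuts, sculpting completes once no original vertices remain in the rebuilt section.
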(event `self.ReceiveBeginPlay`
  (bind _vertices (`KismetProceduralMeshLibrary.GetSectionFromProceduralMesh` (`self.Gem`)))
  (set `self.OriginalVertices` _vertices)
  (if (not (`self.World Geode?`))
    (bind _returnvalue (`|CreateWidget` "/Game/Blueprints/Widgets/SculptModeUI.SculptModeUI_C"))
    (bind _output_get (set `self.SculptUI` _returnvalue))
    (`UserWidget.AddToViewport` _output_get 0)))

(event `self.ReceiveTick`
  (params (DeltaSeconds :type "Float (single-precision)"))
  (bind _returnvalue (`GameplayStatics.GetPlayerController` 0))
  (bind _sculptui (`self.SculptUI`))
  (bind _sculptui_2 (`self.SculptUI`))
  (bind (_locationx _locationy) (`WidgetLayoutLibrary.GetMousePositionScaledByDPI` (`GameplayStatics.GetPlayerController` 0)))
  (bind (_locationx_2 _locationy_2) (`WidgetLayoutLibrary.GetMousePositionScaledByDPI` (`GameplayStatics.GetPlayerController` 0)))
  (if (not (`self.World Geode?`))
    (`self.RotateGeode`))
  (if (`self.Knife Project?`)
    (if (`PlayerController.IsInputKeyDown` _returnvalue "LeftMouseButton")
      ;[1 1 1] Start cut
      (set `/Game/Blueprints/Widgets/SculptModeUI.StartPoint` (`self.mouseDownViewportPosition`) _sculptui_2)
      (set `/Game/Blueprints/Widgets/SculptModeUI.EndPoint` (`KismetMathLibrary.MakeVector2D` _locationx _locationy) _sculptui_2)
      (elif (`PlayerController.WasInputKeyJustReleased` _returnvalue "LeftMouseButton")
        ;[1 1 1] Finish cut
        (`self.KnifeProjectFacetingSlice`)
        (else
          ;[1 1 1] While cutting
          (set `self.mouseDownPosition` (`PlayerController.DeprojectMousePositionToWorld` (`GameplayStatics.GetPlayerController` 0)))
          (set `self.mouseDownViewportPosition` (`KismetMathLibrary.MakeVector2D` _locationx_2 _locationy_2))
          (set `/Game/Blueprints/Widgets/SculptModeUI.StartPoint` (0.0 0.0) _sculptui)
          (set `/Game/Blueprints/Widgets/SculptModeUI.EndPoint` (0.0 0.0) _sculptui))))
    (else
      ;[1 1 1] Non knife project
      (if (`PlayerController.WasInputKeyJustPressed` (`GameplayStatics.GetPlayerController` 0) "LeftMouseButton")
        (if (not (`self.SculptCompleted`))
          (`self.Slice`))))))

(fn `DestroyViewportGeode`
  (`Widget.RemoveFromParent` (`self.SculptUI`))
  (`self.K2_DestroyActor`))

(fn `KnifeProjectFacetingSlice`
  (locals (MouseUpPosition :type "Vector Structure" :default (0.0 0.0 0.0)) (BaseNormal :type "Vector Structure" :default (0.0 0.0 0.0)) (`Geode under cut?` :type Boolean) (MousePositionDifference :type "Vector Structure") (`Player Viewpoint` :type "Vector Structure"))
  (bind _returnvalue (`GameplayStatics.GetPlayerController` 0))
  (bind _player_viewpoint (`local.Player Viewpoint`))
  (bind _gem (`self.Gem`))
  (bind _basenormal (`local.BaseNormal`))
  (bind _mouseupposition (`local.MouseUpPosition`))
  (bind _returnvalue_2 (- (`local.MouseUpPosition`) (`SceneComponent.K2_GetComponentLocation` (`self.Gem`))))
  ;[1 1 1] Variable setup
  (bind _output_get (set `local.MouseUpPosition` (`PlayerController.DeprojectMousePositionToWorld` _returnvalue)))
  (set `local.MousePositionDifference` (- _output_get (`self.mouseDownPosition`)))
  (set `local.Player Viewpoint` (`Controller.GetPlayerViewPoint` _returnvalue))
  (if (> (`KismetMathLibrary.Vector_Distance` (`self.mouseDownPosition`) (`local.MouseUpPosition`)) 1.0)
    ;[1 1 1] Setting normal
    (set `local.BaseNormal` (`KismetMathLibrary.Cross_VectorVector` (- (`local.MouseUpPosition`) _player_viewpoint) (- (`self.mouseDownPosition`) _player_viewpoint)))
    (if (> (`KismetMathLibrary.DegAcos` (/ (`KismetMathLibrary.Dot_VectorVector` _returnvalue_2 _basenormal) (* (`KismetMathLibrary.VSize` _returnvalue_2) (`KismetMathLibrary.VSize` _basenormal)))) 90.0)
      (`KismetProceduralMeshLibrary.SliceProceduralMesh` _gem _mouseupposition (`local.BaseNormal`) false "UseLastSectionForCap" (`self.gemMaterial`))
      (else
        (`KismetProceduralMeshLibrary.SliceProceduralMesh` (`self.Gem`) _mouseupposition (* (`local.BaseNormal`) -1.0) false "UseLastSectionForCap" (`self.gemMaterial`))))
    (bind _vertices (`KismetProceduralMeshLibrary.GetSectionFromProceduralMesh` _gem))
    (`ProceduralMeshComponent.ClearCollisionConvexMeshes` _gem)
    (`ProceduralMeshComponent.AddCollisionConvexMesh` _gem _vertices)))

(fn `RandomSphereSlice`
  (bind _returnvalue (`KismetMathLibrary.Normal` (`KismetMathLibrary.MakeVector` (`KismetMathLibrary.RandomFloatInRange` -1.0 1.0) (`KismetMathLibrary.RandomFloatInRange` -1.0 1.0) (`KismetMathLibrary.RandomFloatInRange` -1.0 1.0))))
  (`KismetProceduralMeshLibrary.SliceProceduralMesh` (`self.Gem`) (+ (+ (`SceneComponent.K2_GetComponentLocation` (`self.Gem`)) (0.0 0.0 50.0)) (* _returnvalue (* (`self.radius`) -1.0))) _returnvalue false "CreateNewSectionForCap"))

(fn `ReconstructProcMesh`
  (params (Verts :type "Array of Vector Structure") (Tris :type "Array of Integer") (Normals :type "Array of Vector Structure") (UVs :type "Array of Vector2D Structure") (Tangents :type "Array of ProcMeshTangent Structure"))
  (bind _gem (`self.Gem`))
  (set `self.tempVerts` Verts)
  (set `self.tempTris` Tris)
  (set `self.tempNormals` Normals)
  (set `self.tempUVs` UVs)
  (set `self.tempTangents` Tangents)
  (`ProceduralMeshComponent.ClearMeshSection` _gem 0)
  (`ProceduralMeshComponent.CreateMeshSection_LinearColor` :`self` _gem :`Vertices` (`self.tempVerts`) :`Triangles` (`self.tempTris`) :`Normals` (`self.tempNormals`) :`UV0` (`self.tempUVs`) :`Tangents` (`self.tempTangents`) :`bCreateCollision` true))

(fn `RefreshMesh`
  (bind _gem (`self.Gem`))
  (bind (_vertices _triangles _normals _uvs _tangents) (`KismetProceduralMeshLibrary.GetSectionFromStaticMesh` (`self.Mesh`)))
  (`ProceduralMeshComponent.CreateMeshSection_LinearColor` :`self` _gem :`Vertices` _vertices :`Triangles` _triangles :`Normals` _normals :`UV0` _uvs :`Tangents` _tangents :`bCreateCollision` true)
  (`PrimitiveComponent.SetMaterial` _gem 0 "/Game/Art/Materials/SubstanceTextures/text_MAT.text_MAT")
  (`StaticMeshComponent.SetStaticMesh` (`self.InnerCollision`) (`self.Mesh`))
  (bind _vertices_2 (`KismetProceduralMeshLibrary.GetSectionFromProceduralMesh` (`self.Gem`)))
  (set `self.OriginalVertices` _vertices_2))

(fn `RotateGeode`
  (bind (_location _rotation) (`Controller.GetPlayerViewPoint` (`GameplayStatics.GetPlayerController` 0)))
  (bind _returnvalue (`WidgetLayoutLibrary.GetMousePositionOnViewport`))
  (if (== (`self.Last Mouse Position`) (0.0 0.0 0.0))
    _
    (elif (`PlayerController.IsInputKeyDown` (`GameplayStatics.GetPlayerController` 0) "RightMouseButton")
      (bind (_returnvalue_x _returnvalue_y) (`KismetMathLibrary.BreakVector` (/ (- (`KismetMathLibrary.MakeVector` (`KismetMathLibrary.BreakVector2D` _returnvalue) (`.Y` (`KismetMathLibrary.BreakVector2D` _returnvalue))) (`self.Last Mouse Position`)) 5.0)))
      (`self.K2_AddActorWorldRotation` (`KismetMathLibrary.MakeRotator` (* (* _returnvalue_y (`KismetMathLibrary.DegSin` (.yaw _rotation))) -1.0) (* _returnvalue_y (`KismetMathLibrary.DegCos` (.yaw _rotation))) (* _returnvalue_x -1.0)))))
  (set `self.Last Mouse Position` (`KismetMathLibrary.MakeVector` (`KismetMathLibrary.BreakVector2D` _returnvalue) (`.Y` (`KismetMathLibrary.BreakVector2D` _returnvalue)))))

(fn `Slice`
  (locals (`myChara Array` :type "Array of Actor Object Reference"))
  (bind _mychara_array (`local.myChara Array`))
  (bind _asmychara (cast `/Game/Blueprints/Important/mychara` (`GameplayStatics.GetPlayerCharacter` 0)))
  (set `local.myChara Array` (`|MakeArray` _asmychara :!type "Actor Object Reference"))
  (if (`self.World Geode?`)
    (`self.SphericalWorldGeodeSlice` _mychara_array)
    (elif (`self.Faceting Geode?`)
      (`self.VerticalFacetingSlice` _mychara_array)
      (else
        (`self.SphericalViewportSlice` _mychara_array))))
  ;[1 1 1] Reconstruct mesh collision
  (bind (_vertices _triangles _normals _uvs _tangents) (`KismetProceduralMeshLibrary.GetSectionFromProceduralMesh` null))
  (`self.ReconstructProcMesh` _vertices _triangles _normals _uvs _tangents)
  (if (not (`self.Faceting Geode?`))
    ;[1 1 1] Sculpt Completion Check
    (set `self.OriginalVertsLeft` 0)
    (for _array_element (`self.OriginalVertices`)
      (if (`KismetArrayLibrary.Array_Contains` (`self.tempVerts`) _array_element)
        (`/Engine/EditorBlueprintResources/StandardMacros.IncrementInt` (`self.OriginalVertsLeft`))))
    (if (< (`self.OriginalVertsLeft`) 1)
      (set `self.SculptCompleted` true)
      (`PrimitiveComponent.SetMaterial` (`self.Gem`) 0 (`self.gemMaterial`))
      (`KismetSystemLibrary.PrintString` "Sculpt done"))))

(fn `SphericalViewportSlice`
  (params (`Actors to Ignore` :type "Array of Actor Object Reference"))
  (bind _location (`Controller.GetPlayerViewPoint` (`GameplayStatics.GetPlayerController` 0)))
  (bind _outhit (`KismetSystemLibrary.LineTraceSingle` _location (+ (* (`.WorldDirection` (`PlayerController.DeprojectMousePositionToWorld` (`GameplayStatics.GetPlayerController` 0))) (555.0 555.0 555.0)) _location) "TraceTypeQuery2" false `Actors to Ignore` "Persistent" false))
  (cast `/Game/Blueprints/GemstoneSystem/Geode` (`.HitActor` (`GameplayStatics.BreakHitResult` _outhit)))
  (bind _returnvalue (- (`.Location` (`GameplayStatics.BreakHitResult` _outhit)) (+ (`SceneComponent.K2_GetComponentLocation` (`self.Gem`)) (`KismetMathLibrary.MakeVector` 0.0 0.0 (`self.radius`)))))
  (`KismetProceduralMeshLibrary.SliceProceduralMesh` (`self.Gem`) (+ (* _returnvalue (-0.1 -0.1 -0.1)) (`.Location` (`GameplayStatics.BreakHitResult` _outhit))) (+ (* _returnvalue (-1.0 -1.0 -1.0)) (`KismetMathLibrary.RandomFloatInRange` -0.1 0.1)) false "CreateNewSectionForCap" (`self.gemMaterial`)))

(fn `SphericalWorldGeodeSlice`
  (params (`Actors to ignore` :type "Array of Actor Object Reference"))
  (bind (_location _rotation) (`Controller.GetPlayerViewPoint` (`GameplayStatics.GetPlayerController` 0)))
  (bind _outhit (`KismetSystemLibrary.LineTraceSingle` _location (+ (* (`KismetMathLibrary.Conv_RotatorToVector` _rotation) (555.0 555.0 555.0)) _location) "TraceTypeQuery2" false `Actors to ignore` "ForOneFrame" false))
  (cast `/Game/Blueprints/GemstoneSystem/Geode` (`.HitActor` (`GameplayStatics.BreakHitResult` _outhit)))
  (bind _returnvalue (- (`.Location` (`GameplayStatics.BreakHitResult` _outhit)) (+ (`SceneComponent.K2_GetComponentLocation` (`self.Gem`)) (`KismetMathLibrary.MakeVector` 0.0 0.0 (`self.radius`)))))
  (`KismetProceduralMeshLibrary.SliceProceduralMesh` (`self.Gem`) (+ (* _returnvalue (-0.1 -0.1 -0.1)) (`.Location` (`GameplayStatics.BreakHitResult` _outhit))) (+ (* _returnvalue (-1.0 -1.0 -1.0)) (`KismetMathLibrary.RandomFloatInRange` -0.1 0.1)) false "UseLastSectionForCap" (`self.gemMaterial`)))

(fn `UserConstructionScript`
  (bind _gem (`self.Gem`))
  (bind (_vertices _triangles _normals _uvs _tangents) (`KismetProceduralMeshLibrary.GetSectionFromStaticMesh` (`self.Mesh`)))
  (`ProceduralMeshComponent.CreateMeshSection_LinearColor` :`self` _gem :`Vertices` _vertices :`Triangles` _triangles :`Normals` _normals :`UV0` _uvs :`Tangents` _tangents :`bCreateCollision` true)
  (`PrimitiveComponent.SetMaterial` _gem 0 (`self.gemMaterial`))
  (`StaticMeshComponent.SetStaticMesh` (`self.InnerCollision`) (`self.Mesh`)))

(fn `VerticalFacetingSlice`
  (params (`Actors to ignore` :type "Array of Actor Object Reference"))
  (bind (_location _rotation) (`Controller.GetPlayerViewPoint` (`GameplayStatics.GetPlayerController` 0)))
  (bind _returnvalue (`KismetMathLibrary.Conv_RotatorToVector` _rotation))
  (bind (_x _y) (`KismetMathLibrary.BreakVector3f` (`KismetMathLibrary.GreaterGreater_VectorRotator` _returnvalue (struct :`Yaw` -90.0))))
  (bind (_x_2 _y_2) (`KismetMathLibrary.BreakVector3f` (`KismetMathLibrary.GreaterGreater_VectorRotator` _returnvalue (struct :`Yaw` 90.0))))
  (bind _returnvalue_2 (`KismetMathLibrary.Normal` (`KismetMathLibrary.MakeVector` _x_2 _y_2)))
  (bind _outhit (`KismetSystemLibrary.LineTraceSingle` _location (+ (* (`.WorldDirection` (`PlayerController.DeprojectMousePositionToWorld` (`GameplayStatics.GetPlayerController` 0))) (555.0 555.0 555.0)) _location) "TraceTypeQuery2" false `Actors to ignore` "Persistent" false))
  (cast `/Game/Blueprints/GemstoneSystem/Geode` (`.HitActor` (`GameplayStatics.BreakHitResult` _outhit)))
  (bind _returnvalue_3 (- (`.Location` (`GameplayStatics.BreakHitResult` _outhit)) (`SceneComponent.K2_GetComponentLocation` (`self.Gem`))))
  (if (> (`KismetMathLibrary.DegAcos` (/ (`KismetMathLibrary.Dot_VectorVector` _returnvalue_3 _returnvalue_2) (* (`KismetMathLibrary.VSize` _returnvalue_3) (`KismetMathLibrary.VSize` _returnvalue_2)))) 90.0)
    (`KismetProceduralMeshLibrary.SliceProceduralMesh` (`self.Gem`) (`.Location` (`GameplayStatics.BreakHitResult` _outhit)) _returnvalue_2 false "CreateNewSectionForCap" (`self.gemMaterial`))
    (else
      (`KismetProceduralMeshLibrary.SliceProceduralMesh` (`self.Gem`) (`.Location` (`GameplayStatics.BreakHitResult` _outhit)) (`KismetMathLibrary.Normal` (`KismetMathLibrary.MakeVector` _x _y)) false "CreateNewSectionForCap" (`self.gemMaterial`)))))