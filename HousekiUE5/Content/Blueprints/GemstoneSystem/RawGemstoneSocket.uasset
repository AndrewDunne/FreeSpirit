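; RawGemstoneSocket is a socket actor that restores its saved raw gemstone when play begins.
; It loads the save game and searches GeodeSocketInfo for the entry matching its ID to recover the gem's mesh, material, mineral name, transform and occupancy.
; If occupied, it spawns a RawGemstone with that data, attaches it snapped to the socket's location and shows its Niagara effect.
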(event `self.ReceiveBeginPlay`
  (bind _current_gem_material (`self.Current Gem Material`))
  (bind _current_gem_mesh (`self.Current Gem Mesh`))
  ;[1 1 1] Load data from savegame
  (bind _returnvalue (`GameplayStatics.LoadGameFromSlot` "mySlot"))
  (bind _asmy_save_game (cast `/Game/Blueprints/Important/mySaveGame` _returnvalue))
  (for _array_element (`/Game/Blueprints/Important/mySaveGame.Geode Socket Info` _asmy_save_game)
    (if (== (break `/Game/Blueprints/Structs/GeodeSocketStruct` _array_element) (`self.ID`))
      (set `self.Current Gem Mesh` (`.GemMesh_29_B39BDFAE454EBA4F03587E96EFE99EE0` (break `/Game/Blueprints/Structs/GeodeSocketStruct` _array_element)))
      (set `self.Current Gem Material` (`.GemMaterial_30_CC2BFD7B438468EA970BCE8F94146615` (break `/Game/Blueprints/Structs/GeodeSocketStruct` _array_element)))
      (set `self.Current Gem Mineral Name` (`.MineralName_32_B1BC1276469986E39B6D0E800CD1D873` (break `/Game/Blueprints/Structs/GeodeSocketStruct` _array_element)))
      (set `self.Current Gem Transform` (`.GemTransform_26_8A77C48341B811BFA3E52E83C342D474` (break `/Game/Blueprints/Structs/GeodeSocketStruct` _array_element)))
      (set `self.HasGem?` (`.HasGem?_25_5C829C4047AB89F7CB5967AFBAF9F473` (break `/Game/Blueprints/Structs/GeodeSocketStruct` _array_element)))))
  (if (`self.HasGem?`)
    (bind _returnvalue_2 (`|SpawnActorFromClass` "/Game/Blueprints/GemstoneSystem/RawGemstone.RawGemstone_C" (`self.Current Gem Transform`) "Undefined" "OverrideRootScale" null null))
    (bind _rawgemstonemesh (`/Game/Blueprints/GemstoneSystem/RawGemstone.RawGemstoneMesh` _returnvalue_2))
    (`PrimitiveComponent.SetMaterial` _rawgemstonemesh 0 _current_gem_material)
    (set `/Game/Blueprints/GemstoneSystem/RawGemstone.Material` _current_gem_material _returnvalue_2)
    (`StaticMeshComponent.SetStaticMesh` _rawgemstonemesh _current_gem_mesh)
    (set `/Game/Blueprints/GemstoneSystem/RawGemstone.Mesh` _current_gem_mesh _returnvalue_2)
    (set `/Game/Blueprints/GemstoneSystem/RawGemstone.Mineral Name` (`self.Current Gem Mineral Name`) _returnvalue_2)
    (`self.K2_AttachToActor` _returnvalue_2 self "None" "SnapToTarget" "KeepRelative" "KeepRelative" true)
    (`SceneComponent.SetVisibility` (`self.Niagara`) true false)))

(fn `UserConstructionScript`)