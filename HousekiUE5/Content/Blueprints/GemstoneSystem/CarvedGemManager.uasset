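; Manager actor for carved gemstones, controlling what appears in gem bowls and on decorative gem stands.
; On BeginPlay it restores the carved geode list and stand decorations from the "mySlot" save, matching stands by ID.
; NewCarvedGem appends a geode, dropping the oldest when the list outgrows the bowls.
; UpdateGemBowls maps list entries to bowls by index, hiding and disabling collision on gem meshes in empty bowls.
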(event `self.ReceiveBeginPlay`
  ;[1 1 1] Loading from SaveGame
  (bind _returnvalue (`GameplayStatics.LoadGameFromSlot` "mySlot"))
  (bind _asmy_save_game (cast `/Game/Blueprints/Important/mySaveGame` _returnvalue))
  (set `self.CarvedGeodes` (`/Game/Blueprints/Important/mySaveGame.Gemstone Bowl Info` _asmy_save_game))
  (`self.UpdateGemBowls`)
  (for _array_element (`/Game/Blueprints/Important/mySaveGame.Gemstone Decor Info` _asmy_save_game)
    (bind _outactors (`GameplayStatics.GetAllActorsOfClass` "/Game/Blueprints/GemstoneSystem/GemStand.GemStand_C"))
    (for _array_element_2 _outactors
      (if (== (`.GemStandID_5_509A3FE94441A1FAB8F51CA24386E91D` (break `/Game/Blueprints/Structs/GemDecorStruct` _array_element)) (`/Game/Blueprints/GemstoneSystem/GemStand.ID` _array_element_2))
        (`/Game/Blueprints/GemstoneSystem/GemStand.Set Gem` _array_element_2 (break `/Game/Blueprints/Structs/GemDecorStruct` _array_element))))))

(fn `NewCarvedGem`
  (params (`New Geode` :type "/Game/Blueprints/Structs/GeodeStruct Structure"))
  (`KismetArrayLibrary.Array_Add` (`self.CarvedGeodes`) `New Geode`)
  (bind _returnvalue (`LayersBlueprintLibrary.GetActors` (`self.GemBowls`)))
  (if (> (`KismetArrayLibrary.Array_Length` (`self.CarvedGeodes`)) (`KismetArrayLibrary.Array_Length` _returnvalue))
    (`KismetArrayLibrary.Array_Remove` (`self.CarvedGeodes`)))
  (`self.UpdateGemBowls`))

(fn `UpdateGemBowls`
  (bind _carvedgeodes (`self.CarvedGeodes`))
  (bind _returnvalue (`LayersBlueprintLibrary.GetActors` (`self.GemBowls`)))
  (for (_array_element _array_index) _returnvalue
    (bind _asgem_bowl (cast `/Game/Blueprints/GemstoneSystem/GemBowl` _array_element))
    (if (<= (`KismetArrayLibrary.Array_Length` _carvedgeodes) _array_index)
      (bind _gemmesh (`/Game/Blueprints/GemstoneSystem/GemBowl.GemMesh` _asgem_bowl))
      (`SceneComponent.SetHiddenInGame` _gemmesh true false)
      (`PrimitiveComponent.SetCollisionEnabled` _gemmesh "NoCollision")
      (set `/Game/Blueprints/GemstoneSystem/GemBowl.hasGem` false _asgem_bowl)
      (else
        (`/Game/Blueprints/GemstoneSystem/GemBowl.Set Gem` _asgem_bowl (`|GetArrayItem` _carvedgeodes _array_index))
        (`SceneComponent.SetHiddenInGame` _gemmesh false false)
        (`PrimitiveComponent.SetCollisionEnabled` _gemmesh "QueryAndPhysics")
        (set `/Game/Blueprints/GemstoneSystem/GemBowl.hasGem` true _asgem_bowl)))))

(fn `UserConstructionScript`)