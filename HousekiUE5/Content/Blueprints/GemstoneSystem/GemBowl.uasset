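; GemBowl is an interactable bowl actor that displays a carved gem and lets the player pick it up.
; It finds the CarvedGemManager on BeginPlay; interacting while it has a gem hands over the CarvedGeodes entry matching its index in GemBowls.
; That entry is then removed and the manager refreshes the bowls.
; SetGem rebuilds the child Gem actor's procedural mesh and material from stored gem data.
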(event `self.ReceiveBeginPlay`
  (bind _outactors (`GameplayStatics.GetAllActorsOfClass` "/Game/Blueprints/GemstoneSystem/CarvedGemManager.CarvedGemManager_C"))
  (for _array_element _outactors
    (set `self.Carved Gem Manager` _array_element)))

(event `/Game/Blueprints/Interact.Interact`
  (bind _carved_gem_manager (`self.Carved Gem Manager`))
  (bind _carvedgeodes (`/Game/Blueprints/GemstoneSystem/CarvedGemManager.CarvedGeodes` _carved_gem_manager))
  (if (`self.hasGem`)
    (bind _returnvalue (`LayersBlueprintLibrary.GetActors` (`/Game/Blueprints/GemstoneSystem/CarvedGemManager.GemBowls` _carved_gem_manager)))
    (for (_array_element _array_index) _returnvalue
      (if (== _array_element self)
        (bind _mychara (`/Game/Blueprints/MyFunctionLibrary.Get myChara`))
        (`/Game/Blueprints/Important/mychara.Player Hold Gem` _mychara (`|GetArrayItem` _carvedgeodes _array_index))
        (`KismetArrayLibrary.Array_Remove` _carvedgeodes _array_index)))
    (`/Game/Blueprints/GemstoneSystem/CarvedGemManager.UpdateGemBowls` (`self.Carved Gem Manager`))))

(fn `Set Gem`
  (params (`Input Gem` :type "/Game/Blueprints/Structs/GeodeStruct Structure"))
  (bind _asgem (cast `/Game/Blueprints/GemstoneSystem/Gem` (`ChildActorComponent.ChildActor` (`self.Gem`))))
  (bind _gemmesh (`/Game/Blueprints/GemstoneSystem/Gem.GemMesh` _asgem))
  (`PrimitiveComponent.SetMaterial` _gemmesh 0 `Input Gem_Material_19_190FE2374252D77EA0E1218E2E757EF7`)
  (`ProceduralMeshComponent.CreateMeshSection_LinearColor` :`self` _gemmesh :`Vertices` `Input Gem_Vertices_3_0148D1AB4DCB098599DD139266253C4A` :`Triangles` `Input Gem_Triangles_9_7A5A8FD44855373EB1E453821F344C33` :`Normals` `Input Gem_Normals_10_B55692DC4A82A6B29B256D9CDE075AD2` :`UV0` `Input Gem_UV0_12_CDF3B10A4BE2B87457BD86BD0CF00F89` :`Tangents` `Input Gem_Tangents_14_70C1D89F4BFA84E8F0C1C78E7608E76B`))

(fn `UserConstructionScript`)