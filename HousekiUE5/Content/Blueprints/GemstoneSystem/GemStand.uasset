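; Display stand actor that holds one gemstone, which the player can place, take or swap by interacting.
; On BeginPlay it restores its gem from the GemstoneDecorInfo entry in the save game matching its ID.
; SetGem rebuilds the gem's procedural mesh and material on a child Gem actor, while RemoveGem clears and hides it.
; The construction script sizes the stand and positions display and gem from Height.
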(event `self.ReceiveBeginPlay`
  (bind _returnvalue (`GameplayStatics.LoadGameFromSlot` "mySlot"))
  (bind _asmy_save_game (cast `/Game/Blueprints/Important/mySaveGame` _returnvalue))
  (for _array_element (`/Game/Blueprints/Important/mySaveGame.Gemstone Decor Info` _asmy_save_game)
    (if (== (`.GemStandID_5_509A3FE94441A1FAB8F51CA24386E91D` (break `/Game/Blueprints/Structs/GemDecorStruct` _array_element)) (`self.ID`))
      (`self.Set Gem` (break `/Game/Blueprints/Structs/GemDecorStruct` _array_element)))))

(event `/Game/Blueprints/Interact.Interact`
  (bind _mychara (`/Game/Blueprints/MyFunctionLibrary.Get myChara`))
  (if (`self.hasGem`)
    (bind _holdinggem_ (`/Game/Blueprints/Important/mychara.HoldingGem?` _mychara))
    (if _holdinggem_
      (bind _heldgem (`/Game/Blueprints/Important/mychara.HeldGem` _mychara))
      (set `self.Temporary gem` _heldgem)
      (`/Game/Blueprints/Important/mychara.Player Hold Gem` _mychara (`self.Gem_`))
      (`self.Remove Gem`)
      (`self.Set Gem` (`self.Temporary gem`))
      (else
        (`/Game/Blueprints/Important/mychara.Player Hold Gem` _mychara (`self.Gem_`))
        (`self.Remove Gem`)))
    (elif _holdinggem_
      (`self.Set Gem` _heldgem)
      (`/Game/Blueprints/Important/mychara.Player Drop Gem` _mychara))))

(fn `Remove Gem`
  (bind _gem (`self.Gem`))
  (bind _asgem (cast `/Game/Blueprints/GemstoneSystem/Gem` (`ChildActorComponent.ChildActor` _gem)))
  (`ProceduralMeshComponent.ClearMeshSection` (`/Game/Blueprints/GemstoneSystem/Gem.GemMesh` _asgem) 0)
  (`SceneComponent.SetVisibility` _gem false true)
  (set `self.hasGem` false))

(fn `Set Gem`
  (params (`Input Gem` :type "/Game/Blueprints/Structs/GeodeStruct Structure"))
  (bind _gem (`self.Gem`))
  (bind _asgem (cast `/Game/Blueprints/GemstoneSystem/Gem` (`ChildActorComponent.ChildActor` _gem)))
  (bind _output_get (set `self.Gem_` `Input Gem`))
  (bind _gemmesh (`/Game/Blueprints/GemstoneSystem/Gem.GemMesh` _asgem))
  (`PrimitiveComponent.SetMaterial` _gemmesh 0 (`.Material_19_190FE2374252D77EA0E1218E2E757EF7` (break `/Game/Blueprints/Structs/GeodeStruct` _output_get)))
  (`ProceduralMeshComponent.CreateMeshSection_LinearColor` :`self` _gemmesh :`Vertices` (break `/Game/Blueprints/Structs/GeodeStruct` _output_get) :`Triangles` (`.Triangles_9_7A5A8FD44855373EB1E453821F344C33` (break `/Game/Blueprints/Structs/GeodeStruct` _output_get)) :`Normals` (`.Normals_10_B55692DC4A82A6B29B256D9CDE075AD2` (break `/Game/Blueprints/Structs/GeodeStruct` _output_get)) :`UV0` (`.UV0_12_CDF3B10A4BE2B87457BD86BD0CF00F89` (break `/Game/Blueprints/Structs/GeodeStruct` _output_get)) :`Tangents` (`.Tangents_14_70C1D89F4BFA84E8F0C1C78E7608E76B` (break `/Game/Blueprints/Structs/GeodeStruct` _output_get)))
  (`SceneComponent.SetVisibility` _gem true true)
  (set `self.hasGem` true))

(fn `UserConstructionScript`
  (bind _returnvalue (* (`self.Height`) 100.0))
  (`SceneComponent.SetRelativeScale3D` (`self.Stand`) (`KismetMathLibrary.MakeVector` 0.15 0.15 (`self.Height`)))
  (`SceneComponent.K2_SetRelativeLocation` (`self.Display`) (`KismetMathLibrary.MakeVector` 0.0 0.0 _returnvalue) false false)
  (`SceneComponent.K2_SetRelativeLocation` (`self.Gem`) (`KismetMathLibrary.MakeVector` 0.0 0.0 (+ _returnvalue 20.0)) false false))