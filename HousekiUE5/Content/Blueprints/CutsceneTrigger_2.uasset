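; Memory cutscene trigger that, when the player character overlaps it after a brief startup grace period, opens a one-shot video clip widget.
; It passes the clip and final transform to the widget but plays the media audio itself, since widgets cannot, fading volume in and out before destroying itself.
; FadeIn and FadeOut events show or hide the trigger's Niagara effect and billboard, scaling billboard brightness by time of day.
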(event `self.ReceiveActorBeginOverlap`
  (params (OtherActor :type "Actor Object Reference"))
  ;[1 1 1] Can't trigger memory in first 3 secs
  (if (> (`GameplayStatics.GetTimeSeconds`) 3.0)
    (if (not (`self.WaitForRepeat`))
      (set `self.WaitForRepeat` true)
      (bind _asmychara (cast `/Game/Blueprints/Important/mychara` OtherActor))
      (set `self.myChara` _asmychara)
      ;[1 1 1] Setting up vid
      (bind _returnvalue (`|CreateWidget` "/Game/Blueprints/Widgets/ClipWidget_2.ClipWidget_2_C"))
      (set `/Game/Blueprints/Widgets/ClipWidget_2.Clip Length` (`self.Clip Length`) _returnvalue)
      (set `/Game/Blueprints/Widgets/ClipWidget_2.FinalLocation` (`SceneComponent.K2_GetComponentLocation` (`self.DefaultSceneRoot`)) _returnvalue)
      (set `/Game/Blueprints/Widgets/ClipWidget_2.FinalRotation` (`self.FinalRotation`) _returnvalue)
      (set `/Game/Blueprints/Widgets/ClipWidget_2.ID` (`self.ID`) _returnvalue)
      (set `/Game/Blueprints/Widgets/ClipWidget_2.MediaSource` (`self.MediaSource`) _returnvalue)
      (`UserWidget.AddToViewport` _returnvalue 0)
      ;[1 1 1] Doing media audio here because widgets can't play media audio
      (`ActorComponent.Activate` (`self.MediaSound`) false)
      (`KismetSystemLibrary.Delay` 1.5)
      (bind (_direction _newtrack_0) (`Timeline|Fade in music` :!via `PlayFromStart`)
        (:`Update`
          (`SynthComponent.SetVolumeMultiplier` (`self.MediaSound`) _newtrack_0))
        (:`Finished`
          (`KismetSystemLibrary.Delay` (- (`self.Clip Length`) 4.0))
          (bind (_direction_2 _newtrack_0_2) (`Timeline|Fade Out Music` :!via `ReverseFromEnd`)
            (:`Update`
              (`SynthComponent.SetVolumeMultiplier` (`self.MediaSound`) _newtrack_0_2))
            (:`Finished`
              (`self.K2_DestroyActor`))))))))

(event `FadeOut`
  (message `AudioParameterControllerInterface.SetFloatParameter` (`self.Niagara`) "SpawnRate" 0.0)
  (bind (_direction _newtrack_0) (`Timeline|Timeline_0` :!via `ReverseFromEnd`)
    (:`Update`
      (bind _asmy_game_state (cast `/Game/Blueprints/Important/myGameState` (`GameplayStatics.GetGameState`)))
      (bind _time_of_day (`/Game/Blueprints/Important/myGameState.GetTimeOfDay` _asmy_game_state))
      (`MaterialInstanceDynamic.SetScalarParameterValue` (`self.BillboardMat`) "Brightness" (* (`/Game/Blueprints/MyMacroLibrary.DayFloatLerps` _time_of_day 0.1 0.2 1.0 1.0 0.7 0.2 0.1) _newtrack_0)))
    (:`Finished`
      (`self.SetActorEnableCollision` false)
      (`self.SetActorHiddenInGame` true))))

(event `FadeIn`
  (`self.SetActorEnableCollision` true)
  (`self.SetActorHiddenInGame` false)
  (message `AudioParameterControllerInterface.SetFloatParameter` (`self.Niagara`) "SpawnRate" 2.0)
  (bind (_direction _newtrack_0) (`Timeline|BillboardFade` :!via `PlayFromStart`)
    (:`Update`
      (bind _asmy_game_state (cast `/Game/Blueprints/Important/myGameState` (`GameplayStatics.GetGameState`)))
      (bind _time_of_day (`/Game/Blueprints/Important/myGameState.GetTimeOfDay` _asmy_game_state))
      (`MaterialInstanceDynamic.SetScalarParameterValue` (`self.BillboardMat`) "Brightness" (* (`/Game/Blueprints/MyMacroLibrary.DayFloatLerps` _time_of_day 0.1 0.2 1.0 1.0 0.7 0.2 0.1) _newtrack_0)))))

(event `self.ReceiveBeginPlay`
  (bind _returnvalue (`KismetMaterialLibrary.CreateDynamicMaterialInstance` "/Game/Art/Materials/VFX/MemoryBillboard_Inst.MemoryBillboard_Inst"))
  (bind _output_get (set `self.BillboardMat` _returnvalue))
  (`PrimitiveComponent.SetMaterial` (`self.MaterialBillboard`) 0 _output_get)
  (if (`KismetStringLibrary.EqualEqual_StrStr` (`self.DayState`) "Day")
    (`MaterialInstanceDynamic.SetScalarParameterValue` _output_get "Brightness" 1.0)
    (elif (`KismetStringLibrary.EqualEqual_StrStr` (`self.DayState`) "Sunset")
      (`MaterialInstanceDynamic.SetScalarParameterValue` _output_get "Brightness" 0.1)
      (elif (`KismetStringLibrary.EqualEqual_StrStr` (`self.DayState`) "Night")
        (`MaterialInstanceDynamic.SetScalarParameterValue` _output_get "Brightness" 0.1)
        (elif (`KismetStringLibrary.EqualEqual_StrStr` (`self.DayState`) "Winter")
          (`MaterialInstanceDynamic.SetScalarParameterValue` _output_get "Brightness" 1.0))))))

(fn `UserConstructionScript`)