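; Moon environment actor that tumbles slowly, with configurable size and brightness.
; The construction script scales the Moon component and feeds MoonBrightness to dynamic materials on Moon and MoonGlow.
; BeginPlay applies a GameTime-based rotation offset, then randomizes angular velocity and overwrites the orientation with a random one.
; Tick adds a tiny fraction of that velocity as local rotation, without delta-time scaling.
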(event `self.ReceiveBeginPlay`
  (bind (_angularvelocity_roll _angularvelocity_pitch _angularvelocity_yaw) (`KismetMathLibrary.BreakRotator` (`self.AngularVelocity`)))
  (bind _asmy_game_state (cast `/Game/Blueprints/Important/myGameState` (`GameplayStatics.GetGameState`)))
  (bind _gametime (`/Game/Blueprints/Important/myGameState.gameTime` _asmy_game_state))
  (`self.K2_AddActorLocalRotation` (`KismetMathLibrary.MakeRotator` (* _angularvelocity_roll _gametime) (* _angularvelocity_pitch _gametime) (* _angularvelocity_yaw _gametime)))
  (set `self.AngularVelocity` (`KismetMathLibrary.RandomRotator` true))
  (`self.K2_SetActorRotation` (`KismetMathLibrary.RandomRotator` true)))

(event `self.ReceiveTick`
  (params (DeltaSeconds :type "Float (single-precision)"))
  (`self.K2_AddActorLocalRotation` (* (`self.AngularVelocity`) 2e-05)))

(fn `UserConstructionScript`
  (`SceneComponent.SetRelativeScale3D` (`self.Moon`) (`KismetMathLibrary.Conv_DoubleToVector` (`self.MoonSize`)))
  (bind _returnvalue (`KismetMaterialLibrary.CreateDynamicMaterialInstance` "/Game/Art/Materials/Sky/Moon.Moon"))
  (`PrimitiveComponent.SetMaterial` (`self.Moon`) 0 _returnvalue)
  (`MaterialInstanceDynamic.SetScalarParameterValue` _returnvalue "MoonBrightness" (`self.MoonBrightness`))
  (bind _returnvalue_2 (`KismetMaterialLibrary.CreateDynamicMaterialInstance` "/Game/Art/Materials/Sky/MoonGlow.MoonGlow"))
  (`PrimitiveComponent.SetMaterial` (`self.MoonGlow`) 0 _returnvalue_2)
  (`MaterialInstanceDynamic.SetScalarParameterValue` _returnvalue_2 "MoonBrightness" (`self.MoonBrightness`)))