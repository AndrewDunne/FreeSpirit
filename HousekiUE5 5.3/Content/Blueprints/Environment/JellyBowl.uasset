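; JellyBowl is an interactable environment prop: a glowing bowl of water and jelly that splashes when the player interacts with it.
; Its construction script applies one Color to the light, dynamic water material and bloom effects, and hides the stand unless HasStand is set.
; Interact spawns a tinted Niagara splash and a triggered 2D sound, then briefly locks out repeats.
; InteractCheck shows the grab crosshair, or the default one during a splash.
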(event `/Game/Blueprints/Interact.InteractCheck`
  (params (`Component Hit` :type "ActorComponent Object Reference"))
  (if (`self.JellyIsSplashing`)
    (bind _icon (`/Game/Blueprints/Widgets/Crosshair.Icon` (`/Game/Blueprints/Important/mychara.Crosshair` (stale _mychara))))
    (`Image.SetBrushFromTexture` _icon (`/Game/Blueprints/Important/mychara.DefaultCrosshair` (stale _mychara)) false)
    (else
      (bind _mychara (`/Game/Blueprints/MyFunctionLibrary.Get myChara`))
      (`Image.SetBrushFromTexture` _icon "/Game/Art/UI/Icons/Grab.Grab" false))))

(event `/Game/Blueprints/Interact.Interact`
  (params (`Component Hit` :type "ActorComponent Object Reference"))
  (if (not (`self.JellyIsSplashing`))
    (set `self.JellyIsSplashing` true)
    (`self.JellySplash`)
    (`KismetSystemLibrary.Delay` 1.0)
    (set `self.JellyIsSplashing` false)))

(fn `JellySplash`
  (bind _returnvalue (`NiagaraFunctionLibrary.SpawnSystemAttached` "/Game/Art/FX/Particles/JellySplash.JellySplash" (`self.bowl-stand-tall`) "Jelly" (0.0 0.0 0.0) (struct) "KeepRelativeOffset" true))
  (`NiagaraComponent.SetVariableLinearColor` _returnvalue "Col" (`self.Color`))
  (bind _returnvalue_2 (`GameplayStatics.SpawnSound2D` "/Game/Sound/Audio_MetaSounds/SFX_MetaSounds/SFX_Foley/SFX_FOL_Splash_Emerge.SFX_FOL_Splash_Emerge" 1.0 1.0 0.0 null))
  (`AudioParameterControllerInterface.SetTriggerParameter` _returnvalue_2 "Splash_Input"))

(fn `UserConstructionScript`
  (`LightComponent.SetLightColor` (`self.PointLight`) (`self.Color`) true)
  (bind _returnvalue (`KismetMaterialLibrary.CreateDynamicMaterialInstance` "/Game/Art/Materials/Water/M_Jellybowl_Water.M_Jellybowl_Water"))
  (bind _output_get (set `self.WaterMat` _returnvalue))
  (`PrimitiveComponent.SetMaterial` (`self.Water`) 0 _output_get)
  (`MaterialInstanceDynamic.SetVectorParameterValue` (`self.WaterMat`) "WaterCol" (`self.Color`))
  (`FXSystemComponent.SetColorParameter` (`self.Bloom_Jelly`) "Color" (`self.Color`))
  (`FXSystemComponent.SetColorParameter` (`self.Bloom_Center`) "Color" (`self.Color`))
  (if (not (`self.HasStand?`))
    (`SceneComponent.SetVisibility` (`self.bowl-stand-tall`) false false)))