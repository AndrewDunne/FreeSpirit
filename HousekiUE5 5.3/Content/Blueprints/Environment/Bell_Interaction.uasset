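; An interactable bell actor that plays a ringing sound at its location when the player interacts with it.
; InteractCheck swaps the character's crosshair to a grab icon while the bell is idle and to the default while it rings.
; Interact sets a ringing flag, spawns the sound and clears the flag after a short delay, blocking repeat rings in the meantime.
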(event `/Game/Blueprints/Interact.InteractCheck`
  (params (`Component Hit` :type "ActorComponent Object Reference"))
  (if (`self.BellIsRinging`)
    (bind _icon (`/Game/Blueprints/Widgets/Crosshair.Icon` (`/Game/Blueprints/Important/mychara.Crosshair` (stale _mychara))))
    (`Image.SetBrushFromTexture` _icon (`/Game/Blueprints/Important/mychara.DefaultCrosshair` (stale _mychara)) false)
    (else
      (bind _mychara (`/Game/Blueprints/MyFunctionLibrary.Get myChara`))
      (`Image.SetBrushFromTexture` _icon "/Game/Art/UI/Icons/Grab.Grab" false))))

(event `/Game/Blueprints/Interact.Interact`
  (params (`Component Hit` :type "ActorComponent Object Reference"))
  (if (not (`self.BellIsRinging`))
    (set `self.BellIsRinging` true)
    (`self.Ring Bell`)
    (`KismetSystemLibrary.Delay` 2.7)
    (set `self.BellIsRinging` false)))

(fn `Ring Bell`
  (`GameplayStatics.SpawnSoundAtLocation` "/Game/Sound/Audio_SoundWaves/SFX_SoundWaves/SFX_Props/SFX_PRP_School/Bell_01.Bell_01" (`self.K2_GetActorLocation`) (struct) 1.0 1.0 0.0 null null))

(fn `UserConstructionScript`)