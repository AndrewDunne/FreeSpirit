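; JellyBowl_MainHall is an environment prop for a glowing jelly bowl with a point light and a colored bloom effect.
; The construction script passes its Color variable to the BloomLarge component.
; On BeginPlay it stores the light's starting intensity as the maximum, then a one-second looping timer scales that by the JellyBrightness scalar from a material parameter collection, so the light follows shared brightness without using Tick.
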(event `self.ReceiveBeginPlay`
  (`parent.ReceiveBeginPlay`)
  (set `self.LightMaxIntensity` (`LightComponentBase.Intensity` (`self.PointLight`)))
  (`KismetSystemLibrary.K2_SetTimer` null "AdjustLightLevel" 1.0 true))

(fn `AdjustLightLevel`
  (bind _returnvalue (`KismetMaterialLibrary.GetScalarParameterValue` "/Game/Art/Materials/ParameterCollections/PropCollection.PropCollection" "JellyBrightness"))
  (`LightComponent.SetIntensity` (`self.PointLight`) (* _returnvalue (`self.LightMaxIntensity`))))

(fn `UserConstructionScript`
  (`parent.UserConstructionScript`)
  (`NiagaraComponent.SetVariableLinearColor` (`self.Bloom_Large`) "Color" (`self.Color`)))