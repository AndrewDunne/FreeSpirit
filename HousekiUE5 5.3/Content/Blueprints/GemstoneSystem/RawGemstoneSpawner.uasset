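; Spawner actor that grows a random gemstone over real time, then places it as a RawGemstone on a socket in its group.
; It rolls area, family and mineral from weighted lists and DataTables, replacing a random socketed gem when all are full.
; A one-second timer updates the growing gem's scale and dirtiness.
; Saved spawn times let Tick catch up on missed spawns at startup, with long absences capped.
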(event `self.ReceiveBeginPlay`
  (bind _returnvalue (`KismetMathLibrary.Now`))
  (bind _growth_time__days_ (`self.Growth time (days)`))
  (set `self.Startup Spawning Done?` false)
  ;[1 1 1] Loading from savegame
  (bind _savegame (`/Game/Blueprints/MyMacroLibrary.LoadMySaveGame`)
    (:`Existing save game`
      (for _array_element (`/Game/Blueprints/Important/mySaveGame.Geode Spawner Info` _savegame)
        (if (== (`self.ID`) (break `/Game/Blueprints/Structs/GemSpawnerStruct` _array_element))
          (bind _output_get (set `self.Next Spawn Time` (`.NextSpawnTime_22_85357504461D46908B6FB898EB7079CF` (break `/Game/Blueprints/Structs/GemSpawnerStruct` _array_element))))
          (set `self.Current Gem Mesh` (`.GemMesh_23_B39BDFAE454EBA4F03587E96EFE99EE0` (break `/Game/Blueprints/Structs/GemSpawnerStruct` _array_element)))
          (set `self.Current Gem Material` (`.GemMaterial_26_4EF6EAF047B2032FDBE05B8A7403A51C` (break `/Game/Blueprints/Structs/GemSpawnerStruct` _array_element)))
          (set `self.Current Gem Transform` (`.GemTransform_30_E189CAEA4046ECA241D5EFA901B740EF` (break `/Game/Blueprints/Structs/GemSpawnerStruct` _array_element)))
          (bind _output_get_2 (set `self.Current Gem Mineral` (`.MineralName_32_B1BC1276469986E39B6D0E800CD1D873` (break `/Game/Blueprints/Structs/GemSpawnerStruct` _array_element))))
          (`self.UpdateVisibleGemstone`)
          (bind _returnvalue_2 (`|GetDataTableRow` "/Game/Blueprints/Data/GemTypeInfo.GemTypeInfo" _output_get_2)
            (:`then`
              (set `self.Growth time (days)` (`.GrowthTime_Days_40_F3ED812B488BF83210DDE7B6B8BF0CA2` (break `/Game/Blueprints/Structs/GemTypeInfoStruct` _returnvalue_2)))
              (bind _difference__hours_ (`/Game/Blueprints/MyFunctionLibrary.SubtractDateTime` _returnvalue _output_get))
              (if (> (/ _difference__hours_ 24.0) (* _growth_time__days_ 3.0))
                (bind _sum__date_ (`/Game/Blueprints/MyFunctionLibrary.AddDateTime` _returnvalue (* _growth_time__days_ -3.0)))
                (set `self.Next Spawn Time` _sum__date_)))))))
    (:`No save game`
      ;[1 1 1] No save game
      (`self.Generate Random Gemstone`)
      (set `self.Next Spawn Time` (`KismetMathLibrary.Now`))))
  (`KismetSystemLibrary.K2_SetTimer` null "Raw Gem Progress" 1.0 true))

(event `self.ReceiveTick`
  (params (DeltaSeconds :type "Float (single-precision)"))
  (if (not (`self.Startup Spawning Done?`))
    (bind _difference__hours_ (`/Game/Blueprints/MyFunctionLibrary.SubtractDateTime` (`KismetMathLibrary.Now`) (`self.Next Spawn Time`)))
    (if (> _difference__hours_ 0.0)
      (`self.Spawn Gemstone`)
      (else
        (set `self.Startup Spawning Done?` true)))))

(fn `Attach to Socket`
  (params (Socket :type "/Game/Blueprints/GemstoneSystem/RawGemstoneSocket Object Reference"))
  (locals (mySocket :type "/Game/Blueprints/GemstoneSystem/RawGemstoneSocket Object Reference") (myGemstone :type "/Game/Blueprints/GemstoneSystem/RawGemstone Object Reference"))
  (bind _current_gem_mesh (`self.Current Gem Mesh`))
  (bind _mygemstone (`local.myGemstone`))
  (bind _current_gem_material (`self.Current Gem Material`))
  (bind _mysocket (`local.mySocket`))
  (bind _rawgemstonemesh (`/Game/Blueprints/GemstoneSystem/RawGemstone.RawGemstoneMesh` _mygemstone))
  (set `local.mySocket` Socket)
  (bind _returnvalue (`|SpawnActorFromClass` "/Game/Blueprints/GemstoneSystem/RawGemstone.RawGemstone_C" (`SceneComponent.GetRelativeTransform` (`self.Gemstone`)) "Undefined" "OverrideRootScale" null null))
  (set `local.myGemstone` _returnvalue)
  (`StaticMeshComponent.SetStaticMesh` _rawgemstonemesh _current_gem_mesh)
  (`PrimitiveComponent.SetMaterial` _rawgemstonemesh 0 _current_gem_material)
  (set `/Game/Blueprints/GemstoneSystem/RawGemstone.Mesh` _current_gem_mesh _mygemstone)
  (set `/Game/Blueprints/GemstoneSystem/RawGemstone.Material` _current_gem_material _mygemstone)
  (set `/Game/Blueprints/GemstoneSystem/RawGemstone.OwningSocket` (`local.mySocket`) _mygemstone)
  (set `/Game/Blueprints/GemstoneSystem/RawGemstone.Mineral Name` (`self.Current Gem Mineral`) (`local.myGemstone`))
  (`self.K2_AttachToActor` (`local.myGemstone`) (`local.mySocket`) "None" "SnapToTarget" "KeepRelative" "KeepRelative" true)
  (set `/Game/Blueprints/GemstoneSystem/RawGemstoneSocket.Current Gem Mineral Name` (`self.Current Gem Mineral`) _mysocket)
  (set `/Game/Blueprints/GemstoneSystem/RawGemstoneSocket.Current Gem Mesh` (`self.Current Gem Mesh`) _mysocket)
  (set `/Game/Blueprints/GemstoneSystem/RawGemstoneSocket.Current Gem Material` (`self.Current Gem Material`) _mysocket)
  (set `/Game/Blueprints/GemstoneSystem/RawGemstoneSocket.Current Gem Transform` (`SceneComponent.GetRelativeTransform` (`self.Gemstone`)) _mysocket))

(fn `Generate Random Gemstone`
  (locals (GemIndex :type Integer) (ProbabilityIncrement :type "Float (double-precision)") (RandomValue :type "Float (double-precision)") (CurrentFamily :type Name) (CurrentArea :type Name) (RolledSuccessfully :type Boolean))
  ;[1 1 1] Rolling area (family)
  (set `local.RandomValue` (`KismetMathLibrary.RandomFloatInRange` 0.0 1.0))
  (for _array_element (`self.Spawn Areas`)
    (bind _output_get (set `local.ProbabilityIncrement` (+ (`.Probability_5_880AA1B04338EA3FADF336A75448B4AC` (break `/Game/Blueprints/Structs/ProbabilityStruct` _array_element)) (`local.ProbabilityIncrement`))))
    (if (> _output_get (`local.RandomValue`))
      (set `local.CurrentArea` (break `/Game/Blueprints/Structs/ProbabilityStruct` _array_element))
      (set `local.RolledSuccessfully` true)
      (break)))
  (if (`local.RolledSuccessfully`)
    (set `local.RolledSuccessfully` false)
    ;[1 1 1] Get family based on area
    (bind _outrownames (`DataTableFunctionLibrary.GetDataTableRowNames` "/Game/Blueprints/Data/GemFamilyInfo.GemFamilyInfo"))
    (for _array_element_2 _outrownames
      (bind _returnvalue (`|GetDataTableRow` "/Game/Blueprints/Data/GemFamilyInfo.GemFamilyInfo" _array_element_2)
        (:`then`
          (if (== (`|GetArrayItem` (`.SpawnAreas_8_C6768C1A4B878FAD4C8607892E0C7D07` (break `/Game/Blueprints/Structs/GemFamilyInfoStruct` _returnvalue))) (`local.CurrentArea`))
            (set `local.CurrentFamily` (break `/Game/Blueprints/Structs/GemFamilyInfoStruct` _returnvalue))))))
    ;[1 1 1] Rolling Gem (based on family)
    (set `local.RandomValue` (`KismetMathLibrary.RandomFloatInRange` 0.0 1.0))
    (set `local.ProbabilityIncrement` 0.0)
    (bind _returnvalue_2 (`|GetDataTableRow` "/Game/Blueprints/Data/GemFamilyInfo.GemFamilyInfo" (`local.CurrentFamily`))
      (:`then`
        (for _array_element_3 (`.Gems_11_3C9EA2404326E3B348E907928E2C26DB` (break `/Game/Blueprints/Structs/GemFamilyInfoStruct` _returnvalue_2))
          (bind _output_get_2 (set `local.ProbabilityIncrement` (+ (`.Probability_5_880AA1B04338EA3FADF336A75448B4AC` (break `/Game/Blueprints/Structs/ProbabilityStruct` _array_element_3)) (`local.ProbabilityIncrement`))))
          (if (> _output_get_2 (`local.RandomValue`))
            (set `self.Current Gem Mineral` (break `/Game/Blueprints/Structs/ProbabilityStruct` _array_element_3))
            (set `local.RolledSuccessfully` true)
            (break)))
        (if (`local.RolledSuccessfully`)
          (set `local.RolledSuccessfully` false)
          ;[1 1 1] Updating visible gem in spawner and spawn time
          (bind _returnvalue_3 (`|GetDataTableRow` "/Game/Blueprints/Data/GemTypeInfo.GemTypeInfo" (`self.Current Gem Mineral`))
            (:`then`
              (set `self.Current Gem Mesh` (`.Mesh_20_AC3E66EA4CF31A009B268BB7875ABCCE` (break `/Game/Blueprints/Structs/GemTypeInfoStruct` _returnvalue_3)))
              (set `self.Current Gem Material` (`.Material_21_64C6CA1245734390DD33A5860CE982A6` (break `/Game/Blueprints/Structs/GemTypeInfoStruct` _returnvalue_3)))
              (set `self.Current Gem Transform` (`KismetMathLibrary.MakeTransform` (0.0 0.0 0.0) (`KismetMathLibrary.RandomRotator` true) (0.25 0.25 0.25)))
              (`self.UpdateVisibleGemstone`)
              (set `self.Growth time (days)` (`.GrowthTime_Days_40_F3ED812B488BF83210DDE7B6B8BF0CA2` (break `/Game/Blueprints/Structs/GemTypeInfoStruct` _returnvalue_3)))
              (`self.Set Next Spawn Time`)))
          (else
            (`KismetSystemLibrary.PrintString` "ERROR: Could not successfully select gem type")))))
    (else
      (`KismetSystemLibrary.PrintString` "ERROR: Could not successfully select gem area"))))

(fn `Raw Gem Progress`
  (locals (GrowthProgress :type "Float (double-precision)"))
  (bind _difference__hours_ (`/Game/Blueprints/MyFunctionLibrary.SubtractDateTime` (`KismetMathLibrary.Now`) (`self.Next Spawn Time`)))
  (set `local.GrowthProgress` (+ (/ (/ _difference__hours_ 24.0) (`self.Growth time (days)`)) 1.0))
  (`MaterialInstanceDynamic.SetScalarParameterValue` (`self.Current Gem Material Dynamic Instance`) "Dirtiness" (- 1.0 (* (`local.GrowthProgress`) 0.5)))
  (`SceneComponent.SetRelativeScale3D` (`self.Gemstone`) (`KismetMathLibrary.Conv_DoubleToVector` (`KismetMathLibrary.FClamp` (+ (/ (`local.GrowthProgress`) 4.0) 0.25) 0.25)))
  (bind _difference__hours__2 (`/Game/Blueprints/MyFunctionLibrary.SubtractDateTime` (`KismetMathLibrary.Now`) (`self.Next Spawn Time`)))
  (if (>= _difference__hours__2 0.0)
    (`self.Spawn Gemstone`)))

(fn `Set Next Spawn Time`
  (bind _sum__date_ (`/Game/Blueprints/MyFunctionLibrary.AddDateTime` (`self.Next Spawn Time`) (* (`self.Growth time (days)`) 24.0)))
  (set `self.Next Spawn Time` _sum__date_))

(fn `Spawn Gemstone`
  (locals (GemSpawned :type Boolean) (Socket :type "/Game/Blueprints/GemstoneSystem/RawGemstoneSocket Object Reference") (CompatibleSockets :type "Array of /Game/Blueprints/GemstoneSystem/RawGemstoneSocket Object Reference"))
  (bind _socket (`local.Socket`))
  (bind _outactors (`GameplayStatics.GetAllActorsOfClass` "/Game/Blueprints/GemstoneSystem/RawGemstoneSocket.RawGemstoneSocket_C"))
  (for _array_element _outactors
    (if (== (`self.SpawnerGroup`) (`/Game/Blueprints/GemstoneSystem/RawGemstoneSocket.SpawnerGroup` _array_element))
      (set `local.Socket` _array_element)
      (if (`local.GemSpawned`)
        _
        (elif (`/Game/Blueprints/GemstoneSystem/RawGemstoneSocket.HasGem?` _array_element)
          (`KismetArrayLibrary.Array_Add` (`local.CompatibleSockets`) (`local.Socket`))
          (else
            ;[1 1 1] Empty socket found
            (set `local.GemSpawned` true)
            (`self.Attach to Socket` _socket)
            (set `/Game/Blueprints/GemstoneSystem/RawGemstoneSocket.HasGem?` true (`local.Socket`))
            (`SceneComponent.SetVisibility` (`/Game/Blueprints/GemstoneSystem/RawGemstoneSocket.Niagara` _socket) true false))))))
  (if (not (`local.GemSpawned`))
    ;[1 1 1] If all sockets were full
    (bind _output_get (set `local.Socket` (`KismetArrayLibrary.Array_Random` (`local.CompatibleSockets`))))
    (for _array_element_2 (`self.GetAttachedActors` _output_get false false)
      (`self.K2_DestroyActor` _array_element_2))
    (`self.Attach to Socket` (`local.Socket`)))
  (`self.Generate Random Gemstone`))

(fn `UpdateVisibleGemstone`
  (bind _gemstone (`self.Gemstone`))
  (`StaticMeshComponent.SetStaticMesh` _gemstone (`self.Current Gem Mesh`))
  (bind _returnvalue (`KismetMaterialLibrary.CreateDynamicMaterialInstance` (`self.Current Gem Material`)))
  (bind _output_get (set `self.Current Gem Material Dynamic Instance` _returnvalue))
  (`MaterialInstanceDynamic.SetScalarParameterValue` _output_get "Dirtiness" 1.0)
  (`PrimitiveComponent.SetMaterial` _gemstone 0 _output_get)
  (`SceneComponent.K2_SetRelativeTransform` (`self.Gemstone`) (`self.Current Gem Transform`) false false))

(fn `UserConstructionScript`)