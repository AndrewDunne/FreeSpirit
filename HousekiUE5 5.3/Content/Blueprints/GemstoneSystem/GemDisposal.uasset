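; GemDisposal is an interactable actor in the gemstone system where the player discards a held gem.
; On interact it plays the gem collect sound with a trigger parameter and calls PlayerDropGem on the player character.
; Its interact check swaps the crosshair to a trash icon while the player holds a gem, otherwise restores the default crosshair.
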(event `self.ReceiveBeginPlay`
  (bind _mychara (`/Game/Blueprints/MyFunctionLibrary.Get myChara`))
  (set `self.My Chara` _mychara))

(event `/Game/Blueprints/Interact.Interact`
  (params (`Component Hit` :type "ActorComponent Object Reference"))
  (bind _returnvalue (`GameplayStatics.SpawnSound2D` "/Game/Sound/Audio_MetaSounds/SFX_MetaSounds/SFX_Props/SFX_PRP_Gems_Collect.SFX_PRP_Gems_Collect" 1.0 1.0 0.0 null))
  (`AudioParameterControllerInterface.SetTriggerParameter` _returnvalue "Gem_Collect")
  (bind _mychara (`/Game/Blueprints/MyFunctionLibrary.Get myChara`))
  (`/Game/Blueprints/Important/mychara.Player Drop Gem` _mychara))

(event `/Game/Blueprints/Interact.InteractCheck`
  (params (`Component Hit` :type "ActorComponent Object Reference"))
  (bind _my_chara (`self.My Chara`))
  (bind _icon (`/Game/Blueprints/Widgets/Crosshair.Icon` (`/Game/Blueprints/Important/mychara.Crosshair` _my_chara)))
  (if (`/Game/Blueprints/Important/mychara.HoldingGem?` _my_chara)
    (`Image.SetBrushFromTexture` _icon "/Game/Art/UI/Icons/Trash.Trash" false)
    (else
      (`Image.SetBrushFromTexture` _icon (`/Game/Blueprints/Important/mychara.DefaultCrosshair` _my_chara) false))))

(fn `UserConstructionScript`)