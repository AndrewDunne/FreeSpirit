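; GemStand is an interactable display pedestal where the player can place, take or swap a held gemstone.
; BeginPlay restores the gem whose saved decor entry matches the stand's ID; InteractCheck updates the crosshair icon for the available action.
; SetGem rebuilds the child Gem actor's procedural mesh from stored geometry and takes its glow color from the GemTypeInfo table.
; The construction script fits the stand and gem position to Height.
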(event `self.ReceiveBeginPlay`
  (bind _mychara (`/Game/Blueprints/MyFunctionLibrary.Get myChara`))
  (set `self.My Chara` _mychara)
  (bind _savegame (`/Game/Blueprints/MyMacroLibrary.LoadMySaveGame`)
    (:`Existing save game`
      (for _array_element (`/Game/Blueprints/Important/mySaveGame.Gemstone Decor Info` _savegame)
        (if (== (`.GemStandID_5_509A3FE94441A1FAB8F51CA24386E91D` (break `/Game/Blueprints/Structs/GemDecorStruct` _array_element)) (`self.ID`))
          (`self.Set Gem` (break `/Game/Blueprints/Structs/GemDecorStruct` _array_element)))))))

(event `/Game/Blueprints/Interact.Interact`
  (params (`Component Hit` :type "ActorComponent Object Reference"))
  (bind _my_chara (`self.My Chara`))
  (bind _holdinggem_ (`/Game/Blueprints/Important/mychara.HoldingGem?` _my_chara))
  (bind _heldgem (`/Game/Blueprints/Important/mychara.HeldGem` _my_chara))
  (if (`self.hasGem`)
    (if _holdinggem_
      (set `self.Temporary gem` _heldgem)
      (`/Game/Blueprints/Important/mychara.Player Drop Gem` _my_chara)
      (`/Game/Blueprints/Important/mychara.Player Hold Gem` _my_chara (`self.Gem_`))
      (`self.Remove Gem`)
      (`self.Set Gem` (`self.Temporary gem`))
      (else
        (`/Game/Blueprints/Important/mychara.Player Hold Gem` _my_chara (`self.Gem_`))
        (`self.Remove Gem`)))
    (bind _returnvalue (`GameplayStatics.SpawnSound2D` "/Game/Sound/Audio_MetaSounds/SFX_MetaSounds/SFX_Props/SFX_PRP_Gems_Collect.SFX_PRP_Gems_Collect" 1.0 1.0 0.0 null :!label _label))
    (`AudioParameterControllerInterface.SetTriggerParameter` _returnvalue "Gem_Collect")
    (elif _holdinggem_
      (`self.Set Gem` _heldgem)
      (`/Game/Blueprints/Important/mychara.Player Drop Gem` _my_chara)
      (goto _label))))

(event `/Game/Blueprints/Interact.InteractCheck`
  (params (`Component Hit` :type "ActorComponent Object Reference"))
  (bind _my_chara (`self.My Chara`))
  (bind _holdinggem_ (`/Game/Blueprints/Important/mychara.HoldingGem?` (`self.My Chara`)))
  (bind _icon (`/Game/Blueprints/Widgets/Crosshair.Icon` (`/Game/Blueprints/Important/mychara.Crosshair` _my_chara)))
  (if (`self.hasGem`)
    (if _holdinggem_
      (`Image.SetBrushFromTexture` _icon "/Game/Art/UI/Icons/GemDisplay.GemDisplay" false :!label _label_2)
      (else
        (`Image.SetBrushFromTexture` _icon "/Game/Art/UI/Icons/Grab.Grab" false)))
    (elif _holdinggem_
      (goto _label_2)
      (else
        (`Image.SetBrushFromTexture` _icon (`/Game/Blueprints/Important/mychara.DefaultCrosshair` _my_chara) false)))))

(fn `Remove Gem`
  (bind _gem (`self.Gem`))
  (bind _asgem (cast `/Game/Blueprints/GemstoneSystem/Gem` (`ChildActorComponent.ChildActor` _gem)))
  (`ProceduralMeshComponent.ClearMeshSection` (`/Game/Blueprints/GemstoneSystem/Gem.GemMesh` _asgem) 0)
  (`SceneComponent.SetVisibility` _gem false true)
  (set `self.hasGem` false))

(fn `Set Gem`
  (params (`Input Gem` :type "/Game/Blueprints/Structs/GeodeStruct Structure"))
  (bind _gem (`self.Gem`))
  (bind _asgem (cast `/Game/Blueprints/GemstoneSystem/Gem` (`ChildActorComponent.ChildActor` _gem)))
  (bind _output_get (set `self.Gem_` `Input Gem`))
  (bind _gemmesh (`/Game/Blueprints/GemstoneSystem/Gem.GemMesh` _asgem))
  (`PrimitiveComponent.SetMaterial` _gemmesh 0 (`.Material_19_190FE2374252D77EA0E1218E2E757EF7` (break `/Game/Blueprints/Structs/GeodeStruct` _output_get)))
  (`ProceduralMeshComponent.CreateMeshSection_LinearColor` :`self` _gemmesh :`Vertices` (break `/Game/Blueprints/Structs/GeodeStruct` _output_get) :`Triangles` (`.Triangles_9_7A5A8FD44855373EB1E453821F344C33` (break `/Game/Blueprints/Structs/GeodeStruct` _output_get)) :`Normals` (`.Normals_10_B55692DC4A82A6B29B256D9CDE075AD2` (break `/Game/Blueprints/Structs/GeodeStruct` _output_get)) :`UV0` (`.UV0_12_CDF3B10A4BE2B87457BD86BD0CF00F89` (break `/Game/Blueprints/Structs/GeodeStruct` _output_get)) :`Tangents` (`.Tangents_14_70C1D89F4BFA84E8F0C1C78E7608E76B` (break `/Game/Blueprints/Structs/GeodeStruct` _output_get)))
  (bind _returnvalue (`|GetDataTableRow` "/Game/Blueprints/Data/GemTypeInfo.GemTypeInfo" (`.MineralName_31_8AFEAFE54500487AED9CE78F34B44BE9` (break `/Game/Blueprints/Structs/GeodeStruct` _output_get)))
    (:`then`
      (`LightComponent.SetLightColor` (`/Game/Blueprints/GemstoneSystem/Gem.Glow` _asgem) (`.GlowColor_22_097500C4438C0DAECE804E9DA5929AEF` (break `/Game/Blueprints/Structs/GemStatsStruct` (`.HeldStats_56_9C019CFB4362B16BF6A3F5939A45520B` (break `/Game/Blueprints/Structs/GemTypeInfoStruct` _returnvalue)))) true)
      (`SceneComponent.SetVisibility` _gem true true)
      (set `self.hasGem` true))))

(fn `UserConstructionScript`
  (bind _returnvalue (* (`self.Height`) 100.0))
  (`SceneComponent.SetRelativeScale3D` (`self.Stand`) (`KismetMathLibrary.MakeVector` 0.15 0.15 (`self.Height`)))
  (`SceneComponent.K2_SetRelativeLocation` (`self.Display`) (`KismetMathLibrary.MakeVector` 0.0 0.0 _returnvalue) false false)
  (`SceneComponent.K2_SetRelativeLocation` (`self.Gem`) (`KismetMathLibrary.MakeVector` 0.0 0.0 (+ _returnvalue 20.0)) false false))