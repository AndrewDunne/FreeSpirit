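; RawGemstone is a collectible gem actor, with glow color looked up from the GemTypeInfo table by mineral name.
; A looping timer spawns a twinkle sound when the player is near.
; Interacting plays collect audio, clears the owning socket and its sparkles, increments the GameState gem count, signals pickup and first discovery, then destroys the actor.
; InteractCheck swaps the crosshair icon depending on whether the player holds a gem.
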(event `self.ReceiveBeginPlay`
  (bind _rawgemstonemesh (`self.RawGemstoneMesh`))
  (`StaticMeshComponent.SetStaticMesh` _rawgemstonemesh (`self.Mesh`))
  (`PrimitiveComponent.SetMaterial` _rawgemstonemesh 0 (`self.Material`))
  (`KismetSystemLibrary.K2_SetTimer` null "ShouldTwinkleBePlaying" 1.0 true)
  (bind _mychara (`/Game/Blueprints/MyFunctionLibrary.Get myChara`))
  (set `self.My Chara` _mychara))

(event `/Game/Blueprints/Interact.Interact`
  (params (`Component Hit` :type "ActorComponent Object Reference"))
  (bind _owningsocket (`self.OwningSocket`))
  (`/Engine/EditorBlueprintResources/StandardMacros.IncrementInt` (`/Game/Blueprints/Important/mychara.currGemID` (`self.My Chara`))
    (:`  `
      (bind _returnvalue (`GameplayStatics.SpawnSound2D` "/Game/Sound/Audio_MetaSounds/SFX_MetaSounds/SFX_Props/SFX_PRP_Gems_Collect.SFX_PRP_Gems_Collect" 1.0 1.0 0.0 null))
      (`AudioParameterControllerInterface.SetTriggerParameter` _returnvalue "Gem_Collect")
      (`AudioComponent.FadeOut` (`self.TwinkleSound`) 1.0 0.0 "Linear")
      ;[1 1 1] Remove gem from socket and remove sparkles
      (set `/Game/Blueprints/GemstoneSystem/RawGemstoneSocket.HasGem?` false _owningsocket)
      (`SceneComponent.SetVisibility` (`/Game/Blueprints/GemstoneSystem/RawGemstoneSocket.Niagara` _owningsocket) false false)
      (bind _mygamestate (`/Game/Blueprints/MyFunctionLibrary.Get myGameState`))
      (bind _geminfo (`/Game/Blueprints/Important/myGameState.GemInfo` _mygamestate))
      ;[1 1 1] Increment gem count in geminfo
      (for (_array_element _array_index) _geminfo
        (if (== (`self.Mineral Name`) (break `/Game/Blueprints/Structs/GemInventoryInfo` _array_element))
          (if (`.Discovered?_7_B2C42FA94EA821131418188DEB483DAC` (break `/Game/Blueprints/Structs/GemInventoryInfo` _array_element))
            (bind _returnvalue_2 (+ (`.NumHolding_6_FD25FABD480955EAED097694EA8A4C85` (break `/Game/Blueprints/Structs/GemInventoryInfo` _array_element)) 1))
            (`KismetArrayLibrary.Array_Set` _geminfo _array_index (make `/Game/Blueprints/Structs/GemInventoryInfo` (break `/Game/Blueprints/Structs/GemInventoryInfo` _array_element) _returnvalue_2 true))
            (else
              (`KismetArrayLibrary.Array_Set` _geminfo _array_index (make `/Game/Blueprints/Structs/GemInventoryInfo` (break `/Game/Blueprints/Structs/GemInventoryInfo` _array_element) _returnvalue_2 true))
              (bind _mygamestate_2 (`/Game/Blueprints/MyFunctionLibrary.Get myGameState`))
              (`/Game/Blueprints/Important/myGameState.newGemDiscovered` _mygamestate_2)))))
      (`/Game/Blueprints/Important/myGameState.gemPickedUp` _mygamestate)
      (`self.K2_DestroyActor`))))

(event `/Game/Blueprints/Interact.InteractCheck`
  (bind _my_chara (`self.My Chara`))
  (bind _icon (`/Game/Blueprints/Widgets/Crosshair.Icon` (`/Game/Blueprints/Important/mychara.Crosshair` _my_chara)))
  (if (`/Game/Blueprints/Important/mychara.HoldingGem?` _my_chara)
    (`Image.SetBrushFromTexture` _icon "/Game/Art/UI/Icons/DotCrosshair.DotCrosshair" false)
    (else
      (`Image.SetBrushFromTexture` _icon "/Game/Art/UI/Icons/Grab.Grab" false))))

(fn `ShouldTwinkleBePlaying`
  (bind _mychara (`/Game/Blueprints/MyFunctionLibrary.Get myChara`))
  (if (< (`KismetMathLibrary.Vector_Distance` (`self.K2_GetActorLocation` _mychara) (`self.K2_GetActorLocation`)) 6000.0)
    (if (not (`KismetSystemLibrary.IsValid` (`self.TwinkleSound`)))
      (bind _returnvalue (`GameplayStatics.SpawnSoundAtLocation` "/Game/Sound/Audio_MetaSounds/SFX_MetaSounds/SFX_Props/SFX_PRP_Gems_Far.SFX_PRP_Gems_Far" (`self.K2_GetActorLocation`) (struct) 1.0 1.0 0.0 null null))
      (set `self.TwinkleSound` _returnvalue))))

(fn `UserConstructionScript`
  (bind _rawgemstonemesh (`self.RawGemstoneMesh`))
  (`StaticMeshComponent.SetStaticMesh` _rawgemstonemesh (`self.Mesh`))
  (`PrimitiveComponent.SetMaterial` _rawgemstonemesh 0 (`self.Material`))
  (bind _returnvalue (`|GetDataTableRow` "/Game/Blueprints/Data/GemTypeInfo.GemTypeInfo" (`self.Mineral Name`))
    (:`then`
      (`LightComponent.SetLightColor` (`self.Glow`) (`.GlowColor_22_097500C4438C0DAECE804E9DA5929AEF` (break `/Game/Blueprints/Structs/GemStatsStruct` (`.HeldStats_56_9C019CFB4362B16BF6A3F5939A45520B` (break `/Game/Blueprints/Structs/GemTypeInfoStruct` _returnvalue)))) true))))