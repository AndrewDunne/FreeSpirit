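; Interactable coffin for one gem type that the player fills piece by piece with matching held gems after collecting the final memory.
; The construction script builds a shared dynamic material from a gem data table and gathers child meshes as pieces.
; Save data and game-state discovery events control piece, fragment and gemstone visibility.
; Each deposit reveals a piece; completion spawns a Niagara soul explosion, then darkens the gem material after a delay.
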(event `self.ReceiveBeginPlay`
  (bind _savegame (`/Game/Blueprints/MyMacroLibrary.LoadMySaveGame`)
    (:`Existing save game`
      (for _array_element (`/Game/Blueprints/Important/mySaveGame.Geode Inventory Info` _savegame)
        (bind (_progresscheckpoints_beginningtutorialdone_ _progresscheckpoints_memorytutorialdone_ _progresscheckpoints_geminventorytutorialdone_ _progresscheckpoints_gemsculptingtutorialdone_ _progresscheckpoints_allmemoriesfound_ _progresscheckpoints_finalmemorycollected_) (break `/Game/Blueprints/Structs/ProgressCheckpointsStruct` (`/Game/Blueprints/Important/mySaveGame.ProgressCheckpoints` _savegame)))
        (bind (_mineralname _numholding _discovered_) (break `/Game/Blueprints/Structs/GemInventoryInfo` _array_element))
        (if (and _progresscheckpoints_finalmemorycollected_ (and _discovered_ (== (`self.GemType`) _mineralname)))
          (`SceneComponent.SetVisibility` (`self.Fragments`) true false)
          (`SceneComponent.SetVisibility` (`self.Gemstone`) true false)))
      (for _array_element_2 (`/Game/Blueprints/Important/mySaveGame.LustrousCoffins` _savegame)
        (if (== (break `/Game/Blueprints/Structs/LustrousCoffinStruct` _array_element_2) (`self.ID`))
          (set `self.PiecesFound` (`.PiecesFound_3_601A37DC43AFB8CDA781A7929F2806A0` (break `/Game/Blueprints/Structs/LustrousCoffinStruct` _array_element_2)))))
      (for (_array_element_3 _array_index) (`self.PiecesFound`)
        (`SceneComponent.SetVisibility` (`|GetArrayItem` (`self.Pieces`) _array_index) _array_element_3 false)))
    (:`No save game`
      _))
  (`self.Update Lustrous Complete`)
  (`self.UpdateGemMatAlive`)
  (bind _mygamestate (`/Game/Blueprints/MyFunctionLibrary.Get myGameState`))
  (add `/Game/Blueprints/Important/myGameState.newGemDiscovered` _mygamestate (delegate `Gem Discovered`))
  (bind _mychara (`/Game/Blueprints/MyFunctionLibrary.Get myChara`))
  (set `self.My Chara` _mychara))

(event `Gem Discovered`
  (params (Mineral :type Name))
  (bind _mygamestate (`/Game/Blueprints/MyFunctionLibrary.Get myGameState` :!label _label))
  (bind (_progresscheckpoints_beginningtutorialdone_ _progresscheckpoints_memorytutorialdone_ _progresscheckpoints_geminventorytutorialdone_ _progresscheckpoints_gemsculptingtutorialdone_ _progresscheckpoints_allmemoriesfound_ _progresscheckpoints_finalmemorycollected_) (break `/Game/Blueprints/Structs/ProgressCheckpointsStruct` (`/Game/Blueprints/Important/myGameState.ProgressCheckpoints` _mygamestate)))
  (if _progresscheckpoints_finalmemorycollected_
    (for _array_element (`/Game/Blueprints/Important/myGameState.GemInfo` _mygamestate)
      (if (and (== (break `/Game/Blueprints/Structs/GemInventoryInfo` _array_element) (`self.GemType`)) (`.Discovered?_7_B2C42FA94EA821131418188DEB483DAC` (break `/Game/Blueprints/Structs/GemInventoryInfo` _array_element)))
        (`SceneComponent.SetVisibility` (`self.Fragments`) true false)
        (`SceneComponent.SetVisibility` (`self.Gemstone`) true false)))))

(event `Final Mem Found`
  (goto _label))

(event `/Game/Blueprints/Interact.Interact`
  (params (`Component Hit` :type "ActorComponent Object Reference"))
  (bind _piecesfound (`self.PiecesFound`))
  (bind _interactable_ (`self.CheckIfInteractable` `Component Hit`))
  (if _interactable_
    (`/Game/Blueprints/Important/mychara.Player Drop Gem` (`self.My Chara`))
    (bind _returnvalue (`GameplayStatics.SpawnSound2D` "/Game/Sound/Audio_MetaSounds/SFX_MetaSounds/SFX_Props/SFX_PRP_Gems_Collect.SFX_PRP_Gems_Collect" 1.0 1.0 0.0 null))
    (`AudioParameterControllerInterface.SetTriggerParameter` _returnvalue "Gem_Collect")
    (for (_array_element _array_index) _piecesfound
      (if (not _array_element)
        (`KismetArrayLibrary.Array_Set` _piecesfound _array_index true)
        (`SceneComponent.SetVisibility` (`|GetArrayItem` (`self.Pieces`) _array_index) true false)
        (break)))
    (`self.Update Lustrous Complete`)
    (if (`self.LustrousComplete?`)
      (`self.SpawnSoulExplosion`)
      (`KismetSystemLibrary.Delay` 5.0)
      (`self.UpdateGemMatAlive`))))

(event `/Game/Blueprints/Interact.InteractCheck`
  (params (`Component Hit` :type "ActorComponent Object Reference"))
  (bind _interactable_ (`self.CheckIfInteractable` `Component Hit`))
  (if _interactable_
    (bind _mychara (`/Game/Blueprints/MyFunctionLibrary.Get myChara`))
    (`Image.SetBrushFromTexture` (`/Game/Blueprints/Widgets/Crosshair.Icon` (`/Game/Blueprints/Important/mychara.Crosshair` _mychara)) "/Game/Art/UI/Icons/GemDisplay.GemDisplay" false)))

(fn `CheckIfInteractable`
  (params (`Component Hit` :type "ActorComponent Object Reference"))
  (returns (`Interactable?` :type Boolean))
  (bind _mygamestate (`/Game/Blueprints/MyFunctionLibrary.Get myGameState`))
  (bind _mychara (`/Game/Blueprints/MyFunctionLibrary.Get myChara`))
  (bind (_progresscheckpoints_beginningtutorialdone_ _progresscheckpoints_memorytutorialdone_ _progresscheckpoints_geminventorytutorialdone_ _progresscheckpoints_gemsculptingtutorialdone_ _progresscheckpoints_allmemoriesfound_ _progresscheckpoints_finalmemorycollected_) (break `/Game/Blueprints/Structs/ProgressCheckpointsStruct` (`/Game/Blueprints/Important/myGameState.ProgressCheckpoints` _mygamestate)))
  (bind (_heldgem_vertices _heldgem_triangles _heldgem_normals _heldgem_uv0 _heldgem_tangents _heldgem_material _heldgem_mineralname) (break `/Game/Blueprints/Structs/GeodeStruct` (`/Game/Blueprints/Important/mychara.HeldGem` _mychara)))
  (return (and (and (and (and (== `Component Hit` (`self.CollisionBox`)) _progresscheckpoints_finalmemorycollected_) (== _heldgem_mineralname (`self.GemType`))) (`/Game/Blueprints/Important/mychara.HoldingGem?` _mychara)) (not (`self.LustrousComplete?`)))))

(fn `SpawnSoulExplosion`
  (bind _returnvalue (`NiagaraFunctionLibrary.SpawnSystemAtLocation` "/Game/Art/FX/Particles/SoulExplosion.SoulExplosion" (.location (`SceneComponent.K2_GetComponentToWorld` (`self.Chara_Complete`))) (.rotation (`SceneComponent.K2_GetComponentToWorld` (`self.Chara_Complete`))) (.scale (`SceneComponent.K2_GetComponentToWorld` (`self.Chara_Complete`)))))
  (`NiagaraComponent.SetVariableStaticMesh` _returnvalue "GemMesh" "/Game/Art/Models/mySphere.mySphere")
  (`NiagaraComponent.SetVariablePosition` _returnvalue "HeartPosition" (`SceneComponent.K2_GetComponentLocation` (`self.Heart`)))
  (`GameplayStatics.SpawnSoundAtLocation` "/Game/Sound/Audio_SoundWaves/SFX_SoundWaves/SFX_Foley/SFX_FOL_Player/SFX_FOL_Gem/Gem_Dissolve_01.Gem_Dissolve_01" (`SceneComponent.K2_GetComponentLocation` (`self.Heart`)) (struct) 1.0 1.0 0.0 null null))

(fn `Update Lustrous Complete`
  (locals (`IncompletePiece?` :type Boolean))
  (for _array_element (`self.PiecesFound`)
    (if (not _array_element)
      (set `local.IncompletePiece?` true)))
  (bind _output_get (set `self.LustrousComplete?` (not (`local.IncompletePiece?`))))
  (if _output_get
    _))

(fn `UpdateGemMatAlive`
  (bind _gemmat (`self.GemMat`))
  (if (`self.LustrousComplete?`)
    (`MaterialInstanceDynamic.SetVectorParameterValue` :`self` _gemmat :`ParameterName` "LivingLightColor")
    (`MaterialInstanceDynamic.SetVectorParameterValue` _gemmat "Surface Color" (struct :`R` 0.010417 :`G` 0.010417 :`B` 0.010417 :`A` 1.0))
    (`MaterialInstanceDynamic.SetVectorParameterValue` :`self` _gemmat :`ParameterName` "Bubble Layer Depths")
    (`MaterialInstanceDynamic.SetScalarParameterValue` _gemmat "FlareStrength" 0.0)))

(fn `UserConstructionScript`
  (bind _gemmat (`self.GemMat`))
  (bind _gemstone (`self.Gemstone`))
  (`StaticMeshComponent.SetStaticMesh` (`self.Coffin`) (`self.Coffin Mesh`))
  (bind _returnvalue (`|GetDataTableRow` "/Game/Blueprints/Data/GemTypeInfo.GemTypeInfo" (`self.GemType`))
    (:`then`
      (bind _returnvalue_2 (`KismetMaterialLibrary.CreateDynamicMaterialInstance` (`.Material_21_64C6CA1245734390DD33A5860CE982A6` (break `/Game/Blueprints/Structs/GemTypeInfoStruct` _returnvalue))))
      (set `self.GemMat` _returnvalue_2)
      (`MaterialInstanceDynamic.SetScalarParameterValue` _returnvalue_2 "LighterTop_Strength" 0.0)
      (`MaterialInstanceDynamic.SetScalarParameterValue` (`self.GemMat`) "LighterTop_Strength" 0.0)
      (`PrimitiveComponent.SetMaterial` (`self.Fragments`) 0 _gemmat)
      (`PrimitiveComponent.SetMaterial` _gemstone 0 _gemmat)
      (`SceneComponent.K2_SetRelativeTransform` _gemstone (`self.GemTransform`) false false)
      (`StaticMeshComponent.SetStaticMesh` _gemstone (`.Mesh_20_AC3E66EA4CF31A009B268BB7875ABCCE` (break `/Game/Blueprints/Structs/GemTypeInfoStruct` _returnvalue)))
      (`SceneComponent.K2_SetRelativeTransform` (`self.SideTable`) (`self.TableTransform`) false false)
      (for _array_element (`SceneComponent.GetChildrenComponents` (`self.Coffin`) false)
        (bind _asstatic_mesh_component (cast `StaticMeshComponent` _array_element))
        (`PrimitiveComponent.SetMaterial` _asstatic_mesh_component 0 (`self.GemMat`))
        (`KismetArrayLibrary.Array_Add` (`self.Pieces`) _asstatic_mesh_component)))))