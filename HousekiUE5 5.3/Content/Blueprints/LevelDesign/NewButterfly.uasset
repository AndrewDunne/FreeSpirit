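; Ambient butterfly actor that flutters and drifts in the level with no gameplay logic.
; BeginPlay loops the Butterfly3_Anim animation on the skeletal mesh and enlarges the mesh.
; Tick adds world offsets from time-based sine waves at a different frequency per axis, plus an oscillating yaw, for a wandering flight path.
; These per-tick deltas are not scaled by delta time, so the motion varies with frame rate.
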(event `self.ReceiveBeginPlay`
  (bind _skeletalmesh (`self.SkeletalMesh`))
  (`SkeletalMeshComponent.PlayAnimation` _skeletalmesh "/Game/Art/Models/Animated/Butterfly3_Anim.Butterfly3_Anim" true)
  (`SceneComponent.SetRelativeScale3D` _skeletalmesh (3.0 3.0 3.0)))

(event `self.ReceiveTick`
  (params (DeltaSeconds :type "Float (single-precision)"))
  (bind _returnvalue (`GameplayStatics.GetTimeSeconds`))
  (bind _skeletalmesh (`self.SkeletalMesh`))
  (`SceneComponent.K2_AddWorldOffset` _skeletalmesh (`KismetMathLibrary.MakeVector` (* (`KismetMathLibrary.Sin` _returnvalue) 0.4) (* (`KismetMathLibrary.Sin` (* _returnvalue 1.3)) 0.5) (* (`KismetMathLibrary.Sin` (* _returnvalue 1.5)) 0.6)) false false)
  (`SceneComponent.K2_AddWorldRotation` _skeletalmesh (`KismetMathLibrary.MakeRotator` 0.0 0.0 (* (`KismetMathLibrary.Sin` (* _returnvalue 1.5)) 4.0)) false false))

(fn `UserConstructionScript`)