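; Level-design spline actor that builds a cliff by deforming a configurable mesh and material along its spline.
; The construction script divides the spline into sections sized by SplineSparseness times the actor's Y scale, adding a collision-enabled spline mesh component for each.
; Start and end points are sampled by distance in local space, with tangents clamped to section length.
; It has no runtime logic.
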(fn `UserConstructionScript`
  (bind (_returnvalue_x _returnvalue_y) (`KismetMathLibrary.BreakVector` (`self.GetActorScale3D`)))
  (bind _spline (`self.Spline`))
  (bind _section_length (`self.Section Length`))
  (bind _returnvalue (* (`self.Loop index`) _section_length))
  (bind _returnvalue_2 (* (+ (`self.Loop index`) 1) _section_length))
  (set `self.Section Length` (* _returnvalue_y (`self.Spline Sparseness`)))
  (bind _output_get (set `self.LastIndex` (`KismetMathLibrary.FTrunc` (/ (`SplineComponent.GetSplineLength` (`self.Spline`)) (`self.Section Length`)))))
  (for _index (range (+ _output_get 1))
    (set `self.Loop index` _index)
    (bind _returnvalue_3 (`AddComponent|NODE_AddSplineMeshComponent-0`))
    (bind _output_get_2 (set `self.CurrentSplineMesh` _returnvalue_3))
    (`StaticMeshComponent.SetStaticMesh` _output_get_2 (`self.Cliff Mesh`))
    (`PrimitiveComponent.SetMaterial` _output_get_2 0 (`self.Cliff Material`))
    (`SplineMeshComponent.SetForwardAxis` (`self.CurrentSplineMesh`) "X" true)
    (`PrimitiveComponent.SetCollisionEnabled` (`self.CurrentSplineMesh`) "QueryAndPhysics")
    (`SplineMeshComponent.SetStartAndEnd` (`self.CurrentSplineMesh`) (`SplineComponent.GetLocationAtDistanceAlongSpline` _spline _returnvalue "Local") (`KismetMathLibrary.ClampVectorSize` (`SplineComponent.GetTangentAtDistanceAlongSpline` _spline _returnvalue "Local") 0.0 (`self.Section Length`)) (`SplineComponent.GetLocationAtDistanceAlongSpline` _spline _returnvalue_2 "Local") (`KismetMathLibrary.ClampVectorSize` (`SplineComponent.GetTangentAtDistanceAlongSpline` _spline _returnvalue_2 "Local") 0.0 (`self.Section Length`)) true)))