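; Cutscene trigger for the final memory pickup, hidden and non-colliding until activated.
; On BeginPlay it checks the save: it activates if all memories are found, or destroys itself if the final memory is already collected.
; Player overlap flags the final memory in game state, notifies every LustrousCoffin, then runs the parent overlap logic.
; BeginPlay skips the parent version and starts its own looping twinkle-check timer.
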(event `self.ReceiveBeginPlay`
  (`KismetSystemLibrary.K2_SetTimer` null "ShouldTwinkleBePlaying" 1.0 true)
  (`self.SetActorHiddenInGame` true)
  (`self.SetActorEnableCollision` false)
  (bind _savegame (`/Game/Blueprints/MyMacroLibrary.LoadMySaveGame`)
    (:`Existing save game`
      (bind (_progresscheckpoints_beginningtutorialdone_ _progresscheckpoints_memorytutorialdone_ _progresscheckpoints_geminventorytutorialdone_ _progresscheckpoints_gemsculptingtutorialdone_ _progresscheckpoints_allmemoriesfound_ _progresscheckpoints_finalmemorycollected_) (break `/Game/Blueprints/Structs/ProgressCheckpointsStruct` (`/Game/Blueprints/Important/mySaveGame.ProgressCheckpoints` _savegame)))
      (if _progresscheckpoints_allmemoriesfound_
        (if _progresscheckpoints_finalmemorycollected_
          (`self.K2_DestroyActor`)
          (else
            (`self.Activate`)))))))

(event `self.ReceiveActorBeginOverlap`
  (params (OtherActor :type "Actor Object Reference"))
  (cast `/Game/Blueprints/Important/mychara` OtherActor)
  (bind _mygamestate (`/Game/Blueprints/MyFunctionLibrary.Get myGameState`))
  (setmembers `/Game/Blueprints/Structs/ProgressCheckpointsStruct` :`StructRef` (`/Game/Blueprints/Important/myGameState.ProgressCheckpoints` _mygamestate) :`FinalMemoryCollected?` true)
  (bind _outactors (`GameplayStatics.GetAllActorsOfClass` "/Game/Blueprints/GemstoneSystem/LustrousCoffin.LustrousCoffin_C"))
  (for _array_element _outactors
    (`/Game/Blueprints/GemstoneSystem/LustrousCoffin.Final Mem Found` _array_element))
  (`parent.ReceiveActorBeginOverlap` OtherActor))

(fn `Activate`
  (`SceneComponent.SetVisibility` (`self.MaterialBillboard`) true false)
  (`self.SetActorHiddenInGame` false)
  (`self.SetActorEnableCollision` true)
  (set `self.Visible` true))

(fn `UserConstructionScript`
  (`parent.UserConstructionScript`))