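; Memory pickup actor that, on player overlap, plays a video clip widget once, fading media audio in and out before destroying itself.
; Media audio runs on the actor because widgets cannot play it.
; FadeIn/FadeOut toggle the glowing billboard, particles and collision, with brightness scaled by time of day.
; A looping timer spawns distance-layered twinkle sounds, and a bulk-collect event records all but a few hardcoded memory IDs.
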(event `self.ReceiveActorBeginOverlap`
  (params (OtherActor :type "Actor Object Reference"))
  (cast `/Game/Blueprints/Important/mychara` OtherActor)
  ;[1 1 1] Can't trigger memory in first 3 secs
  (if (> (`GameplayStatics.GetTimeSeconds`) 3.0)
    (if (not (`self.Trigger Touched?`))
      (set `self.Trigger Touched?` true)
      (bind _returnvalue (`GameplayStatics.SpawnSound2D` "/Game/Sound/Audio_MetaSounds/SFX_MetaSounds/SFX_Props/SFX_PRP_Memories.SFX_PRP_Memories" 1.0 1.0 0.0 null))
      (`AudioParameterControllerInterface.SetTriggerParameter` _returnvalue "Memory_Collect")
      ;[1 1 1] Setting up vid
      (bind _returnvalue_2 (`|CreateWidget` "/Game/Blueprints/Widgets/ClipWidget_2.ClipWidget_2_C"))
      (set `/Game/Blueprints/Widgets/ClipWidget_2.Clip Length` (`self.Clip Length`) _returnvalue_2)
      (set `/Game/Blueprints/Widgets/ClipWidget_2.FinalLocation` (+ (`SceneComponent.K2_GetComponentLocation` (`self.DefaultSceneRoot`)) (0.0 0.0 50.0)) _returnvalue_2)
      (set `/Game/Blueprints/Widgets/ClipWidget_2.FinalRotation` (`self.FinalRotation`) _returnvalue_2)
      (set `/Game/Blueprints/Widgets/ClipWidget_2.ID` (`self.ID`) _returnvalue_2)
      (set `/Game/Blueprints/Widgets/ClipWidget_2.MediaSource` (`self.MediaSource`) _returnvalue_2)
      (`UserWidget.AddToViewport` _returnvalue_2 0)
      ;[1 1 1] Doing media audio here because widgets can't play media audio
      (`ActorComponent.Activate` (`self.MediaSound`) false)
      (`KismetSystemLibrary.Delay` 1.5)
      (bind (_direction _newtrack_0) (`Timeline|Fade in music` :!via `PlayFromStart`)
        (:`Update`
          (`SynthComponent.SetVolumeMultiplier` (`self.MediaSound`) _newtrack_0))
        (:`Finished`
          (`KismetSystemLibrary.Delay` (- (`self.Clip Length`) 4.0))
          (bind (_direction_2 _newtrack_0_2) (`Timeline|Fade Out Music` :!via `ReverseFromEnd`)
            (:`Update`
              (`SynthComponent.SetVolumeMultiplier` (`self.MediaSound`) _newtrack_0_2))
            (:`Finished`
              (`self.K2_DestroyActor`))))))))

(event `CollectAllMemoriesBut2`
  (bind _id (`self.ID`))
  (if (not (or (or (or (== _id "D17") (== _id "W1")) (== _id "D8")) (== "Reconstructing" _id)))
    (bind _mygamestate (`/Game/Blueprints/MyFunctionLibrary.Get myGameState`))
    (`KismetArrayLibrary.Array_Add` (`/Game/Blueprints/Important/myGameState.collectedMemories` _mygamestate) (`self.ID`))
    (`self.K2_DestroyActor`)))

(event `self.ReceiveBeginPlay`
  (`KismetSystemLibrary.K2_SetTimer` null "ShouldTwinkleBePlaying" 1.0 true))

(event `FadeOut`
  (bind _closetwinkle (`self.CloseTwinkle`))
  (bind _fartwinkle (`self.FarTwinkle`))
  (bind _neartwinkle (`self.NearTwinkle`))
  (message `AudioParameterControllerInterface.SetFloatParameter` (`self.Niagara`) "SpawnRate" 0.0)
  (bind (_direction _newtrack_0) (`Timeline|Timeline_0` :!via `ReverseFromEnd`)
    (:`Update`
      (bind _asmy_game_state (cast `/Game/Blueprints/Important/myGameState` (`GameplayStatics.GetGameState`)))
      (bind _time_of_day (`/Game/Blueprints/Important/myGameState.GetTimeOfDay` _asmy_game_state))
      (`MaterialInstanceDynamic.SetScalarParameterValue` (`self.BillboardMat`) "Brightness" (* (* (`/Game/Blueprints/MyMacroLibrary.DayFloatLerps` _time_of_day 0.1 3.0 12.0 12.0 8.0 2.0 1.0 0.2) _newtrack_0) 3.0)))
    (:`Finished`
      (`self.SetActorEnableCollision` false)
      (`self.SetActorHiddenInGame` true)
      (set `self.Visible` false)
      (if (`KismetSystemLibrary.IsValid` _fartwinkle)
        (`AudioComponent.Stop` _fartwinkle))
      (if (`KismetSystemLibrary.IsValid` _neartwinkle)
        (`AudioComponent.Stop` _neartwinkle))
      (if (`KismetSystemLibrary.IsValid` _closetwinkle)
        (`AudioComponent.Stop` _closetwinkle)))))

(event `FadeIn`
  (`self.SetActorEnableCollision` true)
  (`self.SetActorHiddenInGame` false)
  (set `self.Trigger Touched?` false)
  (message `AudioParameterControllerInterface.SetFloatParameter` (`self.Niagara`) "SpawnRate" 2.0)
  (set `self.Visible` true)
  (bind (_direction _newtrack_0) (`Timeline|BillboardFade` :!via `PlayFromStart`)
    (:`Update`
      (bind _asmy_game_state (cast `/Game/Blueprints/Important/myGameState` (`GameplayStatics.GetGameState`)))
      (bind _time_of_day (`/Game/Blueprints/Important/myGameState.GetTimeOfDay` _asmy_game_state))
      (`MaterialInstanceDynamic.SetScalarParameterValue` (`self.BillboardMat`) "Brightness" (* (* (`/Game/Blueprints/MyMacroLibrary.DayFloatLerps` _time_of_day 0.1 3.0 12.0 12.0 8.0 2.0 1.0 0.2) _newtrack_0) 3.0)))))

(event `self.ReceiveTick`
  (params (DeltaSeconds :type "Float (single-precision)"))
  (if (`self.Visible`)
    (bind _mygamestate (`/Game/Blueprints/MyFunctionLibrary.Get myGameState`))
    (bind _time_of_day (`/Game/Blueprints/Important/myGameState.GetTimeOfDay` _mygamestate))
    (`MaterialInstanceDynamic.SetScalarParameterValue` (`self.BillboardMat`) "Brightness" (* (`/Game/Blueprints/MyMacroLibrary.DayFloatLerps` _time_of_day 0.1 3.0 12.0 12.0 8.0 5.0 3.0 0.1) 3.0))))

(fn `ShouldTwinkleBePlaying`
  (if (`self.Visible`)
    (if (not (`self.Trigger Touched?`))
      (bind _mychara (`/Game/Blueprints/MyFunctionLibrary.Get myChara`))
      (if (< (`KismetMathLibrary.Vector_Distance` (`self.K2_GetActorLocation` _mychara) (`self.K2_GetActorLocation`)) 8000.0)
        (if (not (`KismetSystemLibrary.IsValid` (`self.FarTwinkle`)))
          (bind _returnvalue (`GameplayStatics.SpawnSoundAttached` "/Game/Sound/Audio_MetaSounds/SFX_MetaSounds/SFX_Props/SFX_PRP_Memories_Far.SFX_PRP_Memories_Far" (`self.DefaultSceneRoot`) "None" (0.0 0.0 0.0) (struct) "KeepRelativeOffset" false 1.0 1.0 0.0 null null))
          (set `self.FarTwinkle` _returnvalue))
        (bind _mychara_2 (`/Game/Blueprints/MyFunctionLibrary.Get myChara`))
        (if (< (`KismetMathLibrary.Vector_Distance` (`self.K2_GetActorLocation` _mychara_2) (`self.K2_GetActorLocation`)) 3500.0)
          (if (not (`KismetSystemLibrary.IsValid` (`self.NearTwinkle`)))
            (bind _returnvalue_2 (`GameplayStatics.SpawnSoundAttached` "/Game/Sound/Audio_MetaSounds/SFX_MetaSounds/SFX_Props/SFX_PRP_Memories_Near.SFX_PRP_Memories_Near" (`self.DefaultSceneRoot`) "None" (0.0 0.0 0.0) (struct) "KeepRelativeOffset" false 1.0 1.0 0.0 null null))
            (set `self.NearTwinkle` _returnvalue_2)
            (bind _mychara_3 (`/Game/Blueprints/MyFunctionLibrary.Get myChara`))
            (if (< (`KismetMathLibrary.Vector_Distance` (`self.K2_GetActorLocation` _mychara_3) (`self.K2_GetActorLocation`)) 600.0)
              (if (not (`KismetSystemLibrary.IsValid` (`self.CloseTwinkle`)))
                (bind _returnvalue_3 (`GameplayStatics.SpawnSoundAttached` "/Game/Sound/Audio_MetaSounds/SFX_MetaSounds/SFX_Props/SFX_PRP_Memories_Far.SFX_PRP_Memories_Far" (`self.DefaultSceneRoot`) "None" (0.0 0.0 0.0) (struct) "KeepRelativeOffset" false 1.0 1.0 0.0 null null))
                (set `self.CloseTwinkle` _returnvalue_3)))))))))

(fn `UserConstructionScript`
  (bind _returnvalue (`KismetMaterialLibrary.CreateDynamicMaterialInstance` "/Game/Art/Materials/VFX/MemoryBillboard_Inst.MemoryBillboard_Inst"))
  (bind _output_get (set `self.BillboardMat` _returnvalue))
  (`PrimitiveComponent.SetMaterial` (`self.MaterialBillboard`) 0 _output_get))