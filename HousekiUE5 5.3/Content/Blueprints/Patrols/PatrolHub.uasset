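; Interactable patrol hub that runs timed patrol runs and tracks per-patrol completions and fastest times.
; Interacting with no active patrol offers random picks from the PatrolInfo table; interacting after the last point shows results and updates PatrolSaveData.
; Starting gathers matching PatrolPoint actors by index, revealing them one at a time.
; Each completed point moves one of the Table's SceneCapture2D components to the player's camera to snapshot the view.
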(event `self.ReceiveBeginPlay`
  (bind _mychara (`/Game/Blueprints/MyFunctionLibrary.Get myChara`))
  (set `self.My Chara` _mychara)
  (for _array_element (`SceneComponent.GetChildrenComponents` (`self.Table`) false)
    (bind _asscene_capture_component_2d (cast `SceneCaptureComponent2D` _array_element))
    (`KismetArrayLibrary.Array_Add` (`self.Scene captures`) _asscene_capture_component_2d))
  (set `self.CurrentPatrolIndex` 0)
  (bind _savegame (`/Game/Blueprints/MyMacroLibrary.LoadMySaveGame`)
    (:`Existing save game`
      (set `self.Patrol Save Data` (`/Game/Blueprints/Important/mySaveGame.Patrol Save Data` _savegame)))
    (:`No save game`
      (bind _outrownames (`DataTableFunctionLibrary.GetDataTableRowNames` "/Game/Blueprints/Data/PatrolInfo.PatrolInfo"))
      (for _array_element_2 _outrownames
        (bind _returnvalue (`|GetDataTableRow` "/Game/Blueprints/Data/PatrolInfo.PatrolInfo" _array_element_2)
          (:`then`
            (`KismetArrayLibrary.Array_Add` (`self.Patrol Save Data`) (make `/Game/Blueprints/Structs/PatrolSaveDataStruct` (break `/Game/Blueprints/Structs/PatrolInfoStruct` _returnvalue)))))))))

(event `Start Patrol`
  (`KismetSystemLibrary.PrintString` (`KismetStringLibrary.Concat_StrStr` "Starting patrol " (`KismetStringLibrary.Conv_NameToString` (`self.ActivePatrol`))))
  (set `self.CurrentPatrolIndex` 0)
  (`|VariableSetRef` (`self.ActivePatrolPoints`) (`self.EmptyPatrolPointArray`))
  (bind _outactors (`GameplayStatics.GetAllActorsOfClass` "/Game/Blueprints/Patrols/PatrolPoint.PatrolPoint_C"))
  (for _array_element _outactors
    (if (== (`/Game/Blueprints/Patrols/PatrolPoint.Patrol Name` _array_element) (`self.ActivePatrol`))
      (`KismetArrayLibrary.Array_Set` (`self.ActivePatrolPoints`) (`/Game/Blueprints/Patrols/PatrolPoint.Index` _array_element) _array_element)))
  (`KismetArrayLibrary.Array_RemoveItem` (`self.ActivePatrolPoints`))
  (`self.SetActorHiddenInGame` (`|GetArrayItem` (`self.ActivePatrolPoints`)) false)
  (set `self.PatrolStartTime` (`KismetSystemLibrary.GetGameTimeInSeconds`)))

(event `/Game/Blueprints/Interact.Interact`
  (params (`Component Hit` :type "ActorComponent Object Reference"))
  (bind _patrol_save_data (`self.Patrol Save Data`))
  (bind _my_chara (`self.My Chara`))
  (bind _my_chara_2 (`self.My Chara`))
  (bind _returnvalue (- (`KismetSystemLibrary.GetGameTimeInSeconds`) (`self.PatrolStartTime`)))
  (if (== (`self.ActivePatrol`) "None")
    (`/Game/Blueprints/Important/mychara.Switch to Menuing Controls` _my_chara_2)
    (set `/Game/Blueprints/Important/mychara.menuState` "NewEnumerator4" _my_chara_2)
    (bind _returnvalue_2 (`|CreateWidget` "/Game/Blueprints/Widgets/PatrolBegin.PatrolBegin_C"))
    (`UserWidget.AddToViewport` _returnvalue_2 0)
    (set `/Game/Blueprints/Widgets/PatrolBegin.PatrolHub` self _returnvalue_2)
    (set `/Game/Blueprints/Widgets/PatrolBegin.PatrolData` (`self.Patrol Save Data`) _returnvalue_2)
    (`KismetArrayLibrary.Array_Clear` (`self.Temp_Patrols`))
    (bind _outrownames (`DataTableFunctionLibrary.GetDataTableRowNames` "/Game/Blueprints/Data/PatrolInfo.PatrolInfo"))
    (for _array_element _outrownames
      (bind _returnvalue_3 (`|GetDataTableRow` "/Game/Blueprints/Data/PatrolInfo.PatrolInfo" _array_element)
        (:`then`
          (`KismetArrayLibrary.Array_Add` (`self.Temp_Patrols`) (break `/Game/Blueprints/Structs/PatrolInfoStruct` _returnvalue_3)))))
    (bind _patrols (`/Game/Blueprints/Widgets/PatrolBegin.Patrols` _returnvalue_2))
    (for (_ _array_index) _patrols
      (bind _output_get (set `self.Temp_Patrol` (`KismetArrayLibrary.Array_Random` (`self.Temp_Patrols`))))
      (`KismetArrayLibrary.Array_Set` _patrols _array_index _output_get)
      (`KismetArrayLibrary.Array_RemoveItem` (`self.Temp_Patrols`) (`self.Temp_Patrol`)))
    (elif (`self.FinalPoint?`)
      (set `self.FinalPoint?` false)
      (bind _returnvalue_4 (`|CreateWidget` "/Game/Blueprints/Widgets/PatrolResults.PatrolResults_C"))
      (`UserWidget.AddToViewport` _returnvalue_4 0)
      (set `/Game/Blueprints/Widgets/PatrolResults.TimeToComplete` (- (`KismetSystemLibrary.GetGameTimeInSeconds`) (`self.PatrolStartTime`)) _returnvalue_4)
      (set `/Game/Blueprints/Widgets/PatrolResults.Patrol Name` (`self.ActivePatrol`) _returnvalue_4)
      (for (_array_element_2 _array_index_2) _patrol_save_data
        (if (== (`self.ActivePatrol`) (break `/Game/Blueprints/Structs/PatrolSaveDataStruct` _array_element_2))
          (if (or (< _returnvalue (`.FastestTime_8_DC17D48C44FA8298CED9D59DF2C63C98` (break `/Game/Blueprints/Structs/PatrolSaveDataStruct` _array_element_2))) (== (`.FastestTime_8_DC17D48C44FA8298CED9D59DF2C63C98` (break `/Game/Blueprints/Structs/PatrolSaveDataStruct` _array_element_2)) 0.0))
            (bind _returnvalue_5 (+ (`.NumberTimesCompleted_7_985B7E324D3A43A7F3305D92FF678570` (break `/Game/Blueprints/Structs/PatrolSaveDataStruct` _array_element_2)) 1))
            (`KismetArrayLibrary.Array_Set` _patrol_save_data _array_index_2 (make `/Game/Blueprints/Structs/PatrolSaveDataStruct` (break `/Game/Blueprints/Structs/PatrolSaveDataStruct` _array_element_2) _returnvalue_5 _returnvalue))
            (else
              (`KismetArrayLibrary.Array_Set` _patrol_save_data _array_index_2 (make `/Game/Blueprints/Structs/PatrolSaveDataStruct` (break `/Game/Blueprints/Structs/PatrolSaveDataStruct` _array_element_2) _returnvalue_5 (`.FastestTime_8_DC17D48C44FA8298CED9D59DF2C63C98` (break `/Game/Blueprints/Structs/PatrolSaveDataStruct` _array_element_2))))))))
      (`/Game/Blueprints/Important/mychara.Switch to Menuing Controls` _my_chara)
      (set `/Game/Blueprints/Important/mychara.menuState` "NewEnumerator4" _my_chara)
      (set `self.ActivePatrol` "None"))))

(event `/Game/Blueprints/Interact.InteractCheck`
  (params (`Component Hit` :type "ActorComponent Object Reference"))
  (`Image.SetBrushFromTexture` (`/Game/Blueprints/Widgets/Crosshair.Icon` (`/Game/Blueprints/Important/mychara.Crosshair` (`self.My Chara`))) "/Game/Art/UI/Icons/Grab.Grab" false))

(event `Patrol Point Completed`
  (bind _currentpatrolindex (`self.CurrentPatrolIndex`))
  (bind _output (`|GetArrayItem` (`self.Scene captures`) (`self.CurrentPatrolIndex`)))
  (`SceneComponent.K2_SetWorldTransform` _output (`SceneComponent.K2_GetComponentToWorld` (`/Game/Blueprints/Important/mychara.Camera` (`self.My Chara`))) false false)
  (`self.SetActorHiddenInGame` (`|GetArrayItem` (`self.ActivePatrolPoints`) (`self.CurrentPatrolIndex`)) true)
  (`SceneCaptureComponent2D.CaptureScene` _output)
  (`/Engine/EditorBlueprintResources/StandardMacros.IncrementInt` (`self.CurrentPatrolIndex`)
    (:`  `
      (if (< _currentpatrolindex (`KismetArrayLibrary.Array_Length` (`self.ActivePatrolPoints`)))
        (`self.SetActorHiddenInGame` (`|GetArrayItem` (`self.ActivePatrolPoints`) _currentpatrolindex) false)
        (else
          (set `self.FinalPoint?` true))))))

(fn `UserConstructionScript`)