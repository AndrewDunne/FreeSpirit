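; PatrolPoint is an interactable checkpoint actor that the player completes as part of a patrol.
; Its PatrolPointVolume tracks whether the player character is inside, registering entry only while the point is not hidden.
; While inside, InteractCheck shows a watching crosshair, and Interact reports completion to PatrolHub, restores the default crosshair and clears the inside flag.
; The construction script finds the PatrolHub in the level, keeping the last one found.
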(event `self.ReceiveBeginPlay`
  (bind _mychara (`/Game/Blueprints/MyFunctionLibrary.Get myChara`))
  (set `self.My Chara` _mychara))

(event `self.PatrolPointVolume.OnComponentBeginOverlap`
  (params (OverlappedComponent :type "PrimitiveComponent Object Reference") (OtherActor :type "Actor Object Reference") (OtherComp :type "PrimitiveComponent Object Reference") (OtherBodyIndex :type Integer) (bFromSweep :type Boolean) (SweepResult :type "HitResult Structure (by ref)"))
  (cast `/Game/Blueprints/Important/mychara` OtherActor)
  (if (not (`self.bHidden`))
    (set `self.Player is inside?` true)))

(event `self.PatrolPointVolume.OnComponentEndOverlap`
  (params (OverlappedComponent :type "PrimitiveComponent Object Reference") (OtherActor :type "Actor Object Reference") (OtherComp :type "PrimitiveComponent Object Reference") (OtherBodyIndex :type Integer))
  (cast `/Game/Blueprints/Important/mychara` OtherActor)
  (set `self.Player is inside?` false))

(event `/Game/Blueprints/Interact.InteractCheck`
  (params (`Component Hit` :type "ActorComponent Object Reference"))
  (bind _my_chara (`self.My Chara`))
  (bind _icon (`/Game/Blueprints/Widgets/Crosshair.Icon` (`/Game/Blueprints/Important/mychara.Crosshair` _my_chara)))
  (if (`self.Player is inside?`)
    (`Image.SetBrushFromTexture` _icon "/Game/Art/UI/Icons/Watching.Watching" false)
    (else
      (`Image.SetBrushFromTexture` _icon (`/Game/Blueprints/Important/mychara.DefaultCrosshair` _my_chara) false))))

(event `/Game/Blueprints/Interact.Interact`
  (params (`Component Hit` :type "ActorComponent Object Reference"))
  (bind _my_chara (`self.My Chara`))
  (if (`self.Player is inside?`)
    (`/Game/Blueprints/Patrols/PatrolHub.Patrol Point Completed` (`self.Patrol Hub`))
    (`Image.SetBrushFromTexture` (`/Game/Blueprints/Widgets/Crosshair.Icon` (`/Game/Blueprints/Important/mychara.Crosshair` _my_chara)) (`/Game/Blueprints/Important/mychara.DefaultCrosshair` _my_chara) false)
    (set `self.Player is inside?` false)))

(fn `UserConstructionScript`
  (bind _outactors (`GameplayStatics.GetAllActorsOfClass` "/Game/Blueprints/Patrols/PatrolHub.PatrolHub_C"))
  (for _array_element _outactors
    (set `self.Patrol Hub` _array_element)))