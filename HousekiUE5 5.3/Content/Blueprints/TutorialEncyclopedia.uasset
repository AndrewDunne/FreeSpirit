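; Tutorial encyclopedia pickup, a clipboard that destroys itself on BeginPlay if the save shows the beginning tutorial is done.
; Otherwise it applies a dynamic material, highlighted whenever a per-tick view trace hits a tutorial encyclopedia within short range.
; Interact plays a dissolve timeline on that material, then fires EncyclopediaPickedUp and destroys the actor.
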(event `self.ReceiveBeginPlay`
  (bind _returnvalue (`GameplayStatics.LoadGameFromSlot` "mySlot"))
  (bind _asmy_save_game (cast `/Game/Blueprints/Important/mySaveGame` _returnvalue)
    (:`then`
      (bind _tutorialcheckpoints_beginningtutorialdone_ (break `/Game/Blueprints/Structs/TutorialCheckpointsStruct` (`/Game/Blueprints/Important/mySaveGame.TutorialCheckpoints` _asmy_save_game)))
      (if _tutorialcheckpoints_beginningtutorialdone_
        (`self.K2_DestroyActor`)
        (else
          (bind _returnvalue_2 (`KismetMaterialLibrary.CreateDynamicMaterialInstance` "/Game/Art/Materials/Clipboard_TutorialEncyclopedia.Clipboard_TutorialEncyclopedia" :!label _label))
          (bind _output_get (set `self.Clipboard_Mat` _returnvalue_2))
          (`PrimitiveComponent.SetMaterial` (`self.Clipboard`) 0 _output_get))))
    (:`CastFailed`
      (goto _label))))

(event `Dissolve`
  (bind (_direction _thing) (`Timeline|d_solve`)
    (:`Update`
      (`MaterialInstanceDynamic.SetScalarParameterValue` (`self.Clipboard_Mat`) "DissolveFactor" _thing))
    (:`Finished`
      (`self.EncyclopediaPickedUp`)
      (`self.K2_DestroyActor`))))

(event `/Game/Blueprints/Interact.Interact`
  (`self.Dissolve`))

(event `self.ReceiveTick`
  (params (DeltaSeconds :type "Float (single-precision)"))
  (bind (_location _rotation) (`Controller.GetPlayerViewPoint` (`GameplayStatics.GetPlayerController` 0)))
  (bind _mychara (`/Game/Blueprints/MyFunctionLibrary.Get myChara`))
  (bind _outhit (`KismetSystemLibrary.LineTraceSingle` _location (+ _location (* (`KismetMathLibrary.Conv_RotatorToVector` _rotation) 250.0)) "TraceTypeQuery1" false (`|MakeArray` _mychara :!type "Actor Object Reference") "None" false))
  (cast `/Game/Blueprints/TutorialEncyclopedia` (`.HitActor` (`GameplayStatics.BreakHitResult` _outhit))
    (:`then`
      (`MaterialInstanceDynamic.SetScalarParameterValue` (`self.Clipboard_Mat`) "HighlightFAC" 1.0))
    (:`CastFailed`
      (`MaterialInstanceDynamic.SetScalarParameterValue` (`self.Clipboard_Mat`) "HighlightFAC" 0.0))))

(fn `UserConstructionScript`)