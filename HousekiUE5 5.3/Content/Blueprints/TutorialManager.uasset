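; Tutorial manager that triggers first-time tutorials for the game's opening, memories, gem pickup and sculpting.
; On BeginPlay it binds to GameState and encyclopedia events, and plays a tagged startup cutscene unless the save marks the intro done.
; TutorialCheckpoints flags gate handlers that open menus, overlay a sculpting tutorial widget or blend the camera to the bowls.
; Encyclopedia pickup completes the intro, opens Settings and starts saving.
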(event `StartupCutsceneEnd`
  (set `/Game/Blueprints/Important/mychara.controlState` "NewEnumerator0" (`self.myChara`)))

(event `self.ReceiveBeginPlay`
  (bind _tutorialencyclopedia (`self.TutorialEncyclopedia`))
  (bind _gamestate (`self.GameState`))
  (bind _mygamestate (`/Game/Blueprints/MyFunctionLibrary.Get myGameState`))
  (set `self.GameState` _mygamestate)
  (bind _mychara (`/Game/Blueprints/MyFunctionLibrary.Get myChara`))
  (set `self.myChara` _mychara)
  (bind _outactors (`GameplayStatics.GetAllActorsOfClass` "/Game/Blueprints/TutorialEncyclopedia.TutorialEncyclopedia_C"))
  (for _array_element _outactors
    (set `self.TutorialEncyclopedia` _array_element))
  (add `/Game/Blueprints/Important/myGameState.memoryFound` _gamestate (delegate `Memory Found`))
  (add `/Game/Blueprints/Important/myGameState.gemPickedUp` _gamestate (delegate `Gem Picked Up`))
  (add `/Game/Blueprints/Important/myGameState.sculptStarted` _gamestate (delegate `Sculpt Started`))
  (add `/Game/Blueprints/Important/myGameState.sculptFinished` _gamestate (delegate `Sculpt Finished`))
  (if (`KismetSystemLibrary.IsValid` _tutorialencyclopedia)
    (add `/Game/Blueprints/TutorialEncyclopedia.EncyclopediaPickedUp` _tutorialencyclopedia (delegate `Beginning tutorial complete`)))
  (bind _returnvalue (`GameplayStatics.LoadGameFromSlot` "mySlot"))
  (bind _asmy_save_game (cast `/Game/Blueprints/Important/mySaveGame` _returnvalue)
    (:`then`
      (bind _tutorialcheckpoints_beginningtutorialdone_ (break `/Game/Blueprints/Structs/TutorialCheckpointsStruct` (`/Game/Blueprints/Important/mySaveGame.TutorialCheckpoints` _asmy_save_game)))
      (if (not _tutorialcheckpoints_beginningtutorialdone_)
        (bind _outactors_2 (`GameplayStatics.GetAllActorsOfClassWithTag` "/Script/LevelSequence.LevelSequenceActor" "StartupCutscene" :!label _label))
        (for _array_element_2 _outactors_2
          (set `/Game/Blueprints/Important/mychara.controlState` "NewEnumerator2" (`self.myChara`))
          (bind _sequenceplayer (`LevelSequenceActor.SequencePlayer` _array_element_2))
          (`MovieSceneSequencePlayer.Play` _sequenceplayer)
          (add `MovieSceneSequencePlayer.OnFinished` _sequenceplayer (delegate `StartupCutsceneEnd`)))))
    (:`CastFailed`
      (goto _label))))

(event `Memory Found`
  (bind (_tutorialcheckpoints_beginningtutorialdone_ _tutorialcheckpoints_memorytutorialdone_) (break `/Game/Blueprints/Structs/TutorialCheckpointsStruct` (`/Game/Blueprints/Important/myGameState.TutorialCheckpoints` (`self.GameState`))))
  (if (not _tutorialcheckpoints_memorytutorialdone_)
    (`/Game/Blueprints/Important/mychara.ToggleMenu` (`self.myChara`) "NewEnumerator0" "Map")
    (setmembers `/Game/Blueprints/Structs/TutorialCheckpointsStruct` :`StructRef` (`/Game/Blueprints/Important/myGameState.TutorialCheckpoints` (`self.GameState`)) :`MemoryTutorialDone?` true)))

(event `Gem Picked Up`
  (bind _gamestate (`self.GameState`))
  (bind (_tutorialcheckpoints_beginningtutorialdone_ _tutorialcheckpoints_memorytutorialdone_ _tutorialcheckpoints_geminventorytutorialdone_) (break `/Game/Blueprints/Structs/TutorialCheckpointsStruct` (`/Game/Blueprints/Important/myGameState.TutorialCheckpoints` _gamestate)))
  (if (not _tutorialcheckpoints_geminventorytutorialdone_)
    (`/Game/Blueprints/Important/mychara.ToggleMenu` (`self.myChara`) "NewEnumerator0" "Inventory 1")
    (setmembers `/Game/Blueprints/Structs/TutorialCheckpointsStruct` :`StructRef` (`/Game/Blueprints/Important/myGameState.TutorialCheckpoints` _gamestate) :`GemInventoryTutorialDone?` true)))

(event `Sculpt Started`
  (bind (_tutorialcheckpoints_beginningtutorialdone_ _tutorialcheckpoints_memorytutorialdone_ _tutorialcheckpoints_geminventorytutorialdone_ _tutorialcheckpoints_gemsculptingtutorialdone_) (break `/Game/Blueprints/Structs/TutorialCheckpointsStruct` (`/Game/Blueprints/Important/myGameState.TutorialCheckpoints` (`self.GameState`))))
  (if (not _tutorialcheckpoints_gemsculptingtutorialdone_)
    (bind _returnvalue (`|CreateWidget` "/Game/Blueprints/Widgets/SculptTutorialUI.SculptTutorialUI_C"))
    (`UserWidget.AddToViewport` _returnvalue 0)
    (bind _foundwidgets (`WidgetBlueprintLibrary.GetAllWidgetsOfClass` "/Game/Blueprints/Widgets/SculptModeUI.SculptModeUI_C"))
    (for _array_element _foundwidgets
      (bind _output_get (set `/Game/Blueprints/Widgets/SculptTutorialUI.SculptUI` _array_element _returnvalue))
      (`Widget.SetVisibility` _output_get "Hidden"))))

(event `Sculpt Finished`
  (bind _gamestate (`self.GameState`))
  (bind (_tutorialcheckpoints_beginningtutorialdone_ _tutorialcheckpoints_memorytutorialdone_ _tutorialcheckpoints_geminventorytutorialdone_ _tutorialcheckpoints_gemsculptingtutorialdone_) (break `/Game/Blueprints/Structs/TutorialCheckpointsStruct` (`/Game/Blueprints/Important/myGameState.TutorialCheckpoints` _gamestate)))
  (if (not _tutorialcheckpoints_gemsculptingtutorialdone_)
    (`KismetSystemLibrary.PrintString` "Sculpt end tutorial, cam pointing at bowls")
    (setmembers `/Game/Blueprints/Structs/TutorialCheckpointsStruct` :`StructRef` (`/Game/Blueprints/Important/myGameState.TutorialCheckpoints` _gamestate) :`GemSculptingTutorialDone?` true)
    (bind _outactors (`GameplayStatics.GetAllActorsOfClassWithTag` "/Script/Engine.CameraActor" "BowlCam"))
    (for _array_element _outactors
      (`PlayerController.SetViewTargetWithBlend` (`GameplayStatics.GetPlayerController` 0) _array_element 5.0 "VTBlend_EaseInOut" 5.0 false)
      (bind _mychara (`/Game/Blueprints/MyFunctionLibrary.Get myChara`))
      (set `/Game/Blueprints/Important/mychara.controlState` "NewEnumerator2" _mychara)
      (`KismetSystemLibrary.Delay` 9.0)
      (`PlayerController.SetViewTargetWithBlend` (`GameplayStatics.GetPlayerController` 0) (`self.myChara`) 0.0 "VTBlend_EaseInOut" 5.0 false)
      (set `/Game/Blueprints/Important/mychara.controlState` "NewEnumerator0" _mychara))))

(event `Beginning tutorial complete`
  (setmembers `/Game/Blueprints/Structs/TutorialCheckpointsStruct` :`StructRef` (`/Game/Blueprints/Important/myGameState.TutorialCheckpoints` (`self.GameState`)) :`BeginningTutorialDone?` true)
  (bind _mychara (`/Game/Blueprints/MyFunctionLibrary.Get myChara`))
  (`/Game/Blueprints/Important/mychara.ToggleMenu` _mychara "NewEnumerator0" "Settings")
  (bind _mygamestate (`/Game/Blueprints/MyFunctionLibrary.Get myGameState`))
  (`/Game/Blueprints/Important/myGameState.Start Saving` _mygamestate))

(fn `UserConstructionScript`)