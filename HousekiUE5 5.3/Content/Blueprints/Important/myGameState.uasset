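; Game state that owns persistent progress, settings and the game clock for a gemstone game.
; On BeginPlay it reads DevSettings, loads the save slot or runs first-startup setup, then autosaves on a looping timer only in the Island level by gathering data from the character and world actors.
; Time of day and day count derive from real time since first startup.
; Graphics presets set scalability and swap ocean materials.
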(event `self.ReceiveBeginPlay`
  (bind _returnvalue (`|SpawnActorFromClass` "/Game/Blueprints/DevSettings.DevSettings_C" (`KismetMathLibrary.MakeTransform` (0.0 0.0 0.0)) "Undefined" "OverrideRootScale" null null))
  (set `self.DevMode?` (`/Game/Blueprints/DevSettings.DevMode?` _returnvalue))
  (set `self.Set atmosphere manually?` (`/Game/Blueprints/DevSettings.TimePaused?` _returnvalue))
  (set `self.Manual_TimeOfDay` (`/Game/Blueprints/DevSettings.Paused_TimeOfDay` _returnvalue))
  (set `self.LengthOfDay` (`/Game/Blueprints/DevSettings.LengthOfDay` _returnvalue))
  (if (`self.DevMode?`)
    (`KismetSystemLibrary.ExecuteConsoleCommand` "EnableAllScreenMessages" null)
    (else
      (`KismetSystemLibrary.ExecuteConsoleCommand` "DisableAllScreenMessages" null)))
  (bind _returnvalue_2 (`GameplayStatics.LoadGameFromSlot` "mySlot"))
  (bind _asmy_save_game (cast `/Game/Blueprints/Important/mySaveGame` _returnvalue_2)
    (:`then`
      (`GameplayStatics.SetBaseSoundMix` "/Game/Blueprints/MySoundMix.MySoundMix")
      (bind (_settings_volume _settings_graphicslevel) (break `/Game/Blueprints/Structs/SettingsStruct` (`/Game/Blueprints/Important/mySaveGame.Settings` _asmy_save_game)))
      (`self.ChangeGraphicsLevel` _settings_graphicslevel)
      (`GameplayStatics.SetSoundMixClassOverride` "/Game/Blueprints/MySoundMix.MySoundMix" "/Engine/EngineSounds/Master.Master" _settings_volume 1.0 0.0)
      (set `self.Settings` (make `/Game/Blueprints/Structs/SettingsStruct` _settings_volume _settings_graphicslevel))
      (if (`/Game/Blueprints/Important/mySaveGame.newGame` _asmy_save_game)
        (`KismetSystemLibrary.PrintString` "No Saved game" :!label _label)
        (set `self.FirstStartupTime` (`KismetMathLibrary.Now`))
        (bind _outrownames (`DataTableFunctionLibrary.GetDataTableRowNames` "/Game/Blueprints/Data/GemTypeInfo.GemTypeInfo"))
        (for _array_element _outrownames
          (`KismetArrayLibrary.Array_Add` (`self.GemInfo`) (make `/Game/Blueprints/Structs/GemInventoryInfo` _array_element)))
        (else
          (set `self.FirstStartupTime` (`/Game/Blueprints/Important/mySaveGame.First Startup Time` _asmy_save_game))
          (bind _outrownames_2 (`DataTableFunctionLibrary.GetDataTableRowNames` "/Game/Blueprints/Data/GemTypeInfo.GemTypeInfo"))
          (for _array_element_2 _outrownames_2
            (`KismetArrayLibrary.Array_Add` (`self.GemInfo`) (make `/Game/Blueprints/Structs/GemInventoryInfo` _array_element_2)))
          (set `self.GemInfo` (`/Game/Blueprints/Important/mySaveGame.Geode Inventory Info` _asmy_save_game))
          (set `self.collectedMemories` (`/Game/Blueprints/Important/mySaveGame.Collected Memories` _asmy_save_game))
          (set `self.newlyCollectedMemories` (`/Game/Blueprints/Important/mySaveGame.Newly Collected Memories` _asmy_save_game))
          (set `self.ProgressCheckpoints` (`/Game/Blueprints/Important/mySaveGame.ProgressCheckpoints` _asmy_save_game))
          ;[1 1 1] Only save game while in island level
          (bind _returnvalue_3 (`GameplayStatics.GetCurrentLevelName` true :!label _label_2))
          (if (== _returnvalue_3 "Island")
            (`KismetSystemLibrary.K2_SetTimer` null "SaveGame" 3.0 true)))))
    (:`CastFailed`
      (goto _label))))

(event `Start Saving`
  (goto _label_2))

(fn `ChangeGraphicsLevel`
  (params (Level :type "/Game/Blueprints/Enums/graphicsLevels Enum" :default "NewEnumerator0"))
  (bind _settings_volume (break `/Game/Blueprints/Structs/SettingsStruct` (`self.Settings`)))
  (bind _settings_volume_2 (break `/Game/Blueprints/Structs/SettingsStruct` (`self.Settings`)))
  (bind _settings_volume_3 (break `/Game/Blueprints/Structs/SettingsStruct` (`self.Settings`)))
  (bind _settings_volume_4 (break `/Game/Blueprints/Structs/SettingsStruct` (`self.Settings`)))
  (switch `/Game/Blueprints/Enums/graphicsLevels` Level
    (:`NewEnumerator0`
      (bind _returnvalue (`GameUserSettings.GetGameUserSettings`))
      (`GameUserSettings.SetOverallScalabilityLevel` _returnvalue 0)
      (`GameUserSettings.ApplySettings` _returnvalue true)
      (bind _outactors (`GameplayStatics.GetAllActorsOfClassWithTag` "/Script/Engine.StaticMeshActor" "Ocean"))
      (for _array_element _outactors
        (`PrimitiveComponent.SetMaterial` (`StaticMeshActor.StaticMeshComponent` _array_element) 0 "/Game/Art/Materials/Water/Water2_Opaque_Inst.Water2_Opaque_Inst"))
      (set `self.Settings` (make `/Game/Blueprints/Structs/SettingsStruct` _settings_volume_3)))
    (:`NewEnumerator1`
      (bind _returnvalue_2 (`GameUserSettings.GetGameUserSettings`))
      (`GameUserSettings.SetOverallScalabilityLevel` _returnvalue_2 1)
      (`GameUserSettings.ApplySettings` _returnvalue_2 true)
      (bind _outactors_2 (`GameplayStatics.GetAllActorsOfClassWithTag` "/Script/Engine.StaticMeshActor" "Ocean"))
      (for _array_element_2 _outactors_2
        (`PrimitiveComponent.SetMaterial` (`StaticMeshActor.StaticMeshComponent` _array_element_2) 0 "/Game/Art/Materials/Water/Water2_Inst.Water2_Inst"))
      (set `self.Settings` (make `/Game/Blueprints/Structs/SettingsStruct` _settings_volume_4 "NewEnumerator1")))
    (:`NewEnumerator2`
      (bind _returnvalue_3 (`GameUserSettings.GetGameUserSettings`))
      (`GameUserSettings.SetOverallScalabilityLevel` _returnvalue_3 2)
      (`GameUserSettings.ApplySettings` _returnvalue_3 true)
      (bind _outactors_3 (`GameplayStatics.GetAllActorsOfClassWithTag` "/Script/Engine.StaticMeshActor" "Ocean"))
      (for _array_element_3 _outactors_3
        (`PrimitiveComponent.SetMaterial` (`StaticMeshActor.StaticMeshComponent` _array_element_3) 0 "/Game/Art/Materials/Water/Water2_Inst.Water2_Inst"))
      (set `self.Settings` (make `/Game/Blueprints/Structs/SettingsStruct` _settings_volume_2 "NewEnumerator2")))
    (:`NewEnumerator3`
      (bind _returnvalue_4 (`GameUserSettings.GetGameUserSettings`))
      (`GameUserSettings.SetOverallScalabilityLevel` _returnvalue_4 3)
      (`GameUserSettings.ApplySettings` _returnvalue_4 true)
      (set `self.Settings` (make `/Game/Blueprints/Structs/SettingsStruct` _settings_volume "NewEnumerator3")))))

(fn `GetDay`
  (returns (Day :type Integer))
  (bind _difference__hours_ (`/Game/Blueprints/MyFunctionLibrary.SubtractDateTime` (`KismetMathLibrary.Now`) (`self.FirstStartupTime`)))
  (return (`KismetMathLibrary.FFloor` (* _difference__hours_ 4.0))))

(fn `GetTimeOfDay`
  (returns (`Time of Day` :type "Float (double-precision)"))
  (locals (DayFloat :type "Float (double-precision)" :default 1.0))
  (bind _lengthofday (`self.LengthOfDay`))
  (if (and (`self.Set atmosphere manually?`) (`self.DevMode?`))
    (set `local.DayFloat` (`self.Manual_TimeOfDay`))
    (else
      (bind _difference__hours_ (`/Game/Blueprints/MyFunctionLibrary.SubtractDateTime` (`KismetMathLibrary.Now`) (`self.FirstStartupTime`)))
      (set `local.DayFloat` (/ (mod _difference__hours_ _lengthofday) _lengthofday))
      ;[1 1 1] Makes game first start during daytime
      (set `local.DayFloat` (mod (+ (`local.DayFloat`) 0.3) 1.0))))
  (return (`local.DayFloat`)))

(fn `SaveGame`
  (locals (Savegame :type "/Game/Blueprints/Important/mySaveGame Object Reference"))
  (bind _savegame (`local.Savegame`))
  (bind _savegame_2 (`local.Savegame`))
  (bind _geode_socket_info (`/Game/Blueprints/Important/mySaveGame.Geode Socket Info` (`local.Savegame`)))
  (bind _gemstone_decor_info (`/Game/Blueprints/Important/mySaveGame.Gemstone Decor Info` (`local.Savegame`)))
  (bind _geode_spawner_info (`/Game/Blueprints/Important/mySaveGame.Geode Spawner Info` (`local.Savegame`)))
  (bind _returnvalue (`GameplayStatics.GetCurrentLevelName` true))
  (if (`KismetStringLibrary.EqualEqual_StrStr` _returnvalue "Island")
    (bind _returnvalue_2 (`GameplayStatics.CreateSaveGameObject` "/Game/Blueprints/Important/mySaveGame.mySaveGame_C"))
    (set `local.Savegame` _returnvalue_2)
    ;[1 1 1] General Data
    (set `/Game/Blueprints/Important/mySaveGame.First Startup Time` (`self.FirstStartupTime`) (`local.Savegame`))
    (set `/Game/Blueprints/Important/mySaveGame.Player Transform` (`self.GetTransform` (`GameplayStatics.GetPlayerPawn` 0)) (`local.Savegame`))
    ;[1 1 1] Data in myChara
    (bind _asmychara (cast `/Game/Blueprints/Important/mychara` (`GameplayStatics.GetPlayerCharacter` 0)))
    (set `/Game/Blueprints/Important/mySaveGame.Current Gemstone ID` (`/Game/Blueprints/Important/mychara.currGemID` _asmychara) _savegame_2)
    (set `/Game/Blueprints/Important/mySaveGame.HeldGemstone` (`/Game/Blueprints/Important/mychara.HeldGem` _asmychara) _savegame_2)
    (set `/Game/Blueprints/Important/mySaveGame.HoldingGem` (`/Game/Blueprints/Important/mychara.HoldingGem?` _asmychara) _savegame_2)
    ;[1 1 1] Geode spawner data
    (`KismetArrayLibrary.Array_Clear` _geode_spawner_info)
    (bind _outactors (`GameplayStatics.GetAllActorsOfClass` "/Game/Blueprints/GemstoneSystem/RawGemstoneSpawner.RawGemstoneSpawner_C"))
    (for _array_element _outactors
      (`KismetArrayLibrary.Array_Add` _geode_spawner_info (make `/Game/Blueprints/Structs/GemSpawnerStruct` (`/Game/Blueprints/GemstoneSystem/RawGemstoneSpawner.ID` _array_element) (`/Game/Blueprints/GemstoneSystem/RawGemstoneSpawner.Current Gem Mesh` _array_element) (`/Game/Blueprints/GemstoneSystem/RawGemstoneSpawner.Current Gem Material` _array_element) (`/Game/Blueprints/GemstoneSystem/RawGemstoneSpawner.Current Gem Transform` _array_element) (`/Game/Blueprints/GemstoneSystem/RawGemstoneSpawner.Current Gem Mineral` _array_element) (`/Game/Blueprints/GemstoneSystem/RawGemstoneSpawner.Next Spawn Time` _array_element))))
    ;[1 1 1] Geode socket data
    (`KismetArrayLibrary.Array_Clear` _geode_socket_info)
    (bind _outactors_2 (`GameplayStatics.GetAllActorsOfClass` "/Game/Blueprints/GemstoneSystem/RawGemstoneSocket.RawGemstoneSocket_C"))
    (for _array_element_2 _outactors_2
      (`KismetArrayLibrary.Array_Add` _geode_socket_info (make `/Game/Blueprints/Structs/GemSocketStruct` (`/Game/Blueprints/GemstoneSystem/RawGemstoneSocket.ID` _array_element_2) (`/Game/Blueprints/GemstoneSystem/RawGemstoneSocket.Current Gem Mesh` _array_element_2) (`/Game/Blueprints/GemstoneSystem/RawGemstoneSocket.Current Gem Material` _array_element_2) (`/Game/Blueprints/GemstoneSystem/RawGemstoneSocket.Current Gem Mineral Name` _array_element_2) (`/Game/Blueprints/GemstoneSystem/RawGemstoneSocket.Current Gem Transform` _array_element_2) (`/Game/Blueprints/GemstoneSystem/RawGemstoneSocket.HasGem?` _array_element_2))))
    ;[1 1 1] Carved Gems
    (bind _outactors_3 (`GameplayStatics.GetAllActorsOfClass` "/Game/Blueprints/GemstoneSystem/CarvedGemManager.CarvedGemManager_C"))
    (for _array_element_3 _outactors_3
      (set `/Game/Blueprints/Important/mySaveGame.Gemstone Bowl Info` (`/Game/Blueprints/GemstoneSystem/CarvedGemManager.CarvedGeodes` _array_element_3) (`local.Savegame`)))
    ;[1 1 1] Gem Stands
    (`KismetArrayLibrary.Array_Clear` _gemstone_decor_info)
    (bind _outactors_4 (`GameplayStatics.GetAllActorsOfClass` "/Game/Blueprints/GemstoneSystem/GemStand.GemStand_C"))
    (for _array_element_4 _outactors_4
      (if (`/Game/Blueprints/GemstoneSystem/GemStand.hasGem` _array_element_4)
        (`KismetArrayLibrary.Array_Add` _gemstone_decor_info (make `/Game/Blueprints/Structs/GemDecorStruct` (`/Game/Blueprints/GemstoneSystem/GemStand.Gem_` _array_element_4) (`/Game/Blueprints/GemstoneSystem/GemStand.ID` _array_element_4)))))
    ;[1 1 1] Lustrous Coffins
    (bind _outactors_5 (`GameplayStatics.GetAllActorsOfClass` "/Game/Blueprints/GemstoneSystem/LustrousCoffin.LustrousCoffin_C"))
    (for _array_element_5 _outactors_5
      (`KismetArrayLibrary.Array_Add` (`/Game/Blueprints/Important/mySaveGame.LustrousCoffins` (`local.Savegame`)) (make `/Game/Blueprints/Structs/LustrousCoffinStruct` (`/Game/Blueprints/GemstoneSystem/LustrousCoffin.ID` _array_element_5) (`/Game/Blueprints/GemstoneSystem/LustrousCoffin.PiecesFound` _array_element_5))))
    ;[1 1 1] Settings
    (set `/Game/Blueprints/Important/mySaveGame.Settings` (`self.Settings`) (`local.Savegame`))
    (set `/Game/Blueprints/Important/mySaveGame.Geode Inventory Info` (`self.GemInfo`) (`local.Savegame`))
    (set `/Game/Blueprints/Important/mySaveGame.ProgressCheckpoints` (`self.ProgressCheckpoints`) (`local.Savegame`))
    (set `/Game/Blueprints/Important/mySaveGame.newGame` false (`local.Savegame`))
    ;[1 1 1] Memories
    (set `/Game/Blueprints/Important/mySaveGame.Collected Memories` (`self.collectedMemories`) _savegame)
    (set `/Game/Blueprints/Important/mySaveGame.Newly Collected Memories` (`self.newlyCollectedMemories`) _savegame)
    (bind _outactors_6 (`GameplayStatics.GetAllActorsOfClass` "/Game/Blueprints/Patrols/PatrolHub.PatrolHub_C"))
    (for _array_element_6 _outactors_6
      (set `/Game/Blueprints/Important/mySaveGame.Patrol Save Data` (`/Game/Blueprints/Patrols/PatrolHub.Patrol Save Data` _array_element_6) (`local.Savegame`)))
    (`GameplayStatics.SaveGameToSlot` (`local.Savegame`) "mySlot")))

(fn `Update Game Time`)

(fn `UserConstructionScript`)