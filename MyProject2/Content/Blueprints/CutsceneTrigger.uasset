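; CutsceneTrigger is an overlap trigger actor that plays a video cutscene when the mychara character enters it.
; It stops the character's jog, shows a ClipWidget configured with the clip's media and material, then opens the source after a delay.
; Near the clip's end, a delayed loop fades out the sound, then moves the player to the actor's root and sets FinalRotation.
; A WaitForRepeat flag blocks retriggering until a short cooldown ends.
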(event `self.ReceiveActorBeginOverlap`
  (params (OtherActor :type "Actor Object Reference"))
  (bind _mediasource (`self.MediaSource`))
  (bind _mediaplayer (`self.MediaPlayer`))
  (if (not (`self.WaitForRepeat`))
    (set `self.WaitForRepeat` true)
    (bind _asmychara (cast `/Game/MyStuff/mychara` OtherActor))
    (set `/Game/MyStuff/mychara.JogPressed` false _asmychara)
    (bind _returnvalue (`|CreateWidget` "/Game/Blueprints/ClipWidget.ClipWidget_C"))
    (set `/Game/Blueprints/ClipWidget.Clip Length` (`self.Clip Length`) _returnvalue)
    (set `/Game/Blueprints/ClipWidget.MediaPlayer` _mediaplayer _returnvalue)
    (set `/Game/Blueprints/ClipWidget.MediaSource` _mediasource _returnvalue)
    (`Image.SetBrushFromMaterial` (`/Game/Blueprints/ClipWidget.Image_0` _returnvalue) (`self.Clip Material`))
    (`UserWidget.AddToViewport` _returnvalue 0)
    (`KismetSystemLibrary.Delay` 2.0)
    (`MediaPlayer.OpenSource` _mediaplayer _mediasource)
    (`MediaSoundComponent.SetMediaPlayer` (`self.MediaSound`) _mediaplayer)
    (`KismetSystemLibrary.Delay` (- (`self.Clip Length`) 1.0))
    (`/Game/Blueprints/MyMacroLibrary.ForLoopWithDelay` 0 49 0.01
      (:`loopBody`
        (bind _output_get (set `self.Volume` (- (`self.Volume`) 0.02)))
        (`SynthComponent.SetVolumeMultiplier` (`self.MediaSound`) _output_get))
      (:`completed`
        (`self.K2_SetActorLocation` (`GameplayStatics.GetPlayerPawn` 0) (`SceneComponent.K2_GetComponentLocation` (`self.DefaultSceneRoot`)) false false)
        (`Controller.SetControlRotation` (`GameplayStatics.GetPlayerController` 0) (`self.FinalRotation`))
        (`KismetSystemLibrary.Delay` 3.0)
        (set `self.WaitForRepeat` false)))))

(fn `UserConstructionScript`)